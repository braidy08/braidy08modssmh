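; Controller for the Heist Jukebox mod, which sets up soundtrack selection and saves the player's music options.
; On BeginPlay it loads songs into a shared persistent soundtrack object, restores saved settings and binds to lobby state changes and save requests.
; Lobby events create the pre-heist or jukebox widget and reset heist defaults.
; Playlists persist as soft class references, matched back to loaded tracks on load, with invalid entries pruned.
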(event Custom|JoinedLobbyEvent
  (Widget|RemovefromParent (Variables|Default|GetPreHeistWidget))
  (Variables|/Game/Mods/braidy08mods/HeistJukeboxRecode/HeistSoundtrackPersistentObject.HeistSoundtrackPersistentObject_C|SetJukeboxDisabled (Variables|Default|GetAs%20Heist%20Soundtrack%20Persistent%20Object) false)
  (CallFunction|SetDefaultforHeist)
  (bind _returnvalue (UserInterface|CreateWidget "/Game/Mods/braidy08mods/HeistJukeboxRecode/Widgets/JukeboxWidget.JukeboxWidget_C"))
  (UserInterface|Viewport|AddtoViewport _returnvalue 9999))

(event Custom|ExitedLobbyEvent
  (bind _returnvalue (UserInterface|CreateWidget "/Game/Mods/braidy08mods/HeistJukeboxRecode/Widgets/JukeboxPreHeistWidget.JukeboxPreHeistWidget_C"))
  (UserInterface|Viewport|AddtoViewport _returnvalue 9999)
  (Variables|Default|SetPreHeistWidget _returnvalue))

(event Custom|CallSaveGame
  (CallFunction|Save))

(event EventBeginPlay
  (bind _returnvalue (Class|SBZGameStateMachineFunctionLibrary|GetGameStateMachine))
  (bind _persistentobject (Utilities|GetPersistentObject)
    (:Found
      (Variables|Default|SetAs%20Heist%20Soundtrack%20Persistent%20Object _persistentobject)
      (bind _initalsong (CallFunction|LoadSongs))
      (Variables|/Game/Mods/braidy08mods/HeistJukeboxRecode/HeistSoundtrackPersistentObject.HeistSoundtrackPersistentObject_C|SetPDAHeist (Variables|Default|GetAs%20Heist%20Soundtrack%20Persistent%20Object) _initalsong)
      (CallFunction|SetupSave)
      (EventDispatchers|BindEventtoOnStateMachineEnteredLobby _returnvalue (EventDispatchers|CreateEvent :!event Custom|JoinedLobbyEvent))
      (EventDispatchers|BindEventtoOnStateMachineExitedLobby _returnvalue (EventDispatchers|CreateEvent :!event Custom|ExitedLobbyEvent))
      (CallFunction|ExitedLobbyEvent)
      (EventDispatchers|BindEventtoCallSaveGame (Variables|Default|GetAs%20Heist%20Soundtrack%20Persistent%20Object) (EventDispatchers|CreateEvent :!event Custom|CallSaveGame)))
    (:NotFound
      (CallFunction|PrinttoModLoader "FAILED TO FIND HEIST SOUNDTRACK OBJECT"))))

(fn ConstructionScript)

(fn SetupSave
  (bind _returnvalue (SaveGame|DoesSaveGameExist "HeistJukeboxSaveGame"))
  (if _returnvalue
    (bind _returnvalue_2 (SaveGame|LoadGamefromSlot "HeistJukeboxSaveGame"))
    (bind _asheist_jukebox_save_game (Utilities|Casting|CastToHeistJukeboxSaveGame _returnvalue_2)
      (:then
        (Variables|Default|SetSaveGameObject _asheist_jukebox_save_game)
        (CallFunction|LoadSave)
        (if (Variables|Default|GetSaveLoaded)
          (CallFunction|PrinttoModLoader "save loaded")
          (else
            (SaveGame|DeleteGameinSlot "HeistJukeboxSaveGame" :!label _label)
            (Variables|Default|SetSaveLoaded true)
            (CallFunction|PrinttoModLoader "save doesnt exist loading" :!label _label_2)
            (bind _returnvalue_3 (SaveGame|CreateSaveGameObject "/Game/Mods/braidy08mods/HeistJukeboxRecode/HeistJukeboxSaveGame.HeistJukeboxSaveGame_C"))
            (bind _output_get (Variables|Default|SetSaveGameObject _returnvalue_3))
            (Variables|/Game/Mods/braidy08mods/HeistJukeboxRecode/HeistJukeboxSaveGame.HeistJukeboxSaveGame_C|SetExists _output_get true)
            (SaveGame|SaveGametoSlot _output_get "HeistJukeboxSaveGame"))))
      (:CastFailed
        (CallFunction|PrinttoModLoader "savegame cast failed")
        (goto _label)))
    (else
      (goto _label_2))))

(fn LoadSave
  (bind _savegameobject (Variables|Default|GetSaveGameObject))
  (bind _as_heist_soundtrack_persistent_object (Variables|Default|GetAs%20Heist%20Soundtrack%20Persistent%20Object))
  (bind _savegameobject_2 (Variables|Default|GetSaveGameObject))
  (bind _as_heist_soundtrack_persistent_object_2 (Variables|Default|GetAs%20Heist%20Soundtrack%20Persistent%20Object))
  (bind _pdaheistplaylistarray (Variables|/Game/Mods/braidy08mods/HeistJukeboxRecode/HeistJukeboxSaveGame.HeistJukeboxSaveGame_C|GetPDAHeistPlaylistArray _savegameobject))
  ;[1 1 1] loads all those variables that are supposed to be saved
  (Variables|Default|SetSaveLoaded (Variables|/Game/Mods/braidy08mods/HeistJukeboxRecode/HeistJukeboxSaveGame.HeistJukeboxSaveGame_C|GetExists _savegameobject_2))
  (bind _output_get (Variables|/Game/Mods/braidy08mods/HeistJukeboxRecode/HeistSoundtrackPersistentObject.HeistSoundtrackPersistentObject_C|SetrandomSong _as_heist_soundtrack_persistent_object_2 (Variables|/Game/Mods/braidy08mods/HeistJukeboxRecode/HeistJukeboxSaveGame.HeistJukeboxSaveGame_C|GetRandomEnabled _savegameobject_2)))
  (bind _output_get_2 (Variables|/Game/Mods/braidy08mods/HeistJukeboxRecode/HeistSoundtrackPersistentObject.HeistSoundtrackPersistentObject_C|SetassaultRandomSong _as_heist_soundtrack_persistent_object_2 (Variables|/Game/Mods/braidy08mods/HeistJukeboxRecode/HeistJukeboxSaveGame.HeistJukeboxSaveGame_C|GetRandomAssaultEnabled _savegameobject_2)))
  (bind _output_get_3 (Variables|/Game/Mods/braidy08mods/HeistJukeboxRecode/HeistSoundtrackPersistentObject.HeistSoundtrackPersistentObject_C|SetplaylistEnabled _as_heist_soundtrack_persistent_object_2 (Variables|/Game/Mods/braidy08mods/HeistJukeboxRecode/HeistJukeboxSaveGame.HeistJukeboxSaveGame_C|GetPlaylistEnabled _savegameobject_2)))
  (bind _output_get_4 (Variables|/Game/Mods/braidy08mods/HeistJukeboxRecode/HeistSoundtrackPersistentObject.HeistSoundtrackPersistentObject_C|SetdisableRTCFix _as_heist_soundtrack_persistent_object_2 (Variables|/Game/Mods/braidy08mods/HeistJukeboxRecode/HeistJukeboxSaveGame.HeistJukeboxSaveGame_C|GetRTCFixDisabled _savegameobject_2)))
  (bind _output_get_5 (Variables|/Game/Mods/braidy08mods/HeistJukeboxRecode/HeistSoundtrackPersistentObject.HeistSoundtrackPersistentObject_C|SetEnableRTCStealth _as_heist_soundtrack_persistent_object_2 (Variables|/Game/Mods/braidy08mods/HeistJukeboxRecode/HeistJukeboxSaveGame.HeistJukeboxSaveGame_C|GetRTCStealthEnabled _savegameobject_2)))
  (bind _output_get_6 (Variables|/Game/Mods/braidy08mods/HeistJukeboxRecode/HeistSoundtrackPersistentObject.HeistSoundtrackPersistentObject_C|SetEnableEndlessRanTrack _as_heist_soundtrack_persistent_object_2 (Variables|/Game/Mods/braidy08mods/HeistJukeboxRecode/HeistJukeboxSaveGame.HeistJukeboxSaveGame_C|GetEnableEndlessRanTrack _savegameobject_2)))
  (if (Variables|/Game/Mods/braidy08mods/HeistJukeboxRecode/HeistSoundtrackPersistentObject.HeistSoundtrackPersistentObject_C|GetplaylistEnabled _as_heist_soundtrack_persistent_object_2)
    (for _array_element _pdaheistplaylistarray
      (if (Utilities|IsValidSoftClassReference _array_element)
        (bind _returnvalue (Utilities|LoadClassAssetBlocking _array_element))
        (if (Utilities|IsValidClass _returnvalue)
          (for _array_element_2 (Variables|/Game/Mods/braidy08mods/HeistJukeboxRecode/HeistSoundtrackPersistentObject.HeistSoundtrackPersistentObject_C|GetPDAHeistSoundtrackarray _as_heist_soundtrack_persistent_object)
            (if (== (Utilities|GetClass _array_element_2) _returnvalue)
              ;[1 1 1] makes the thing not shoot up the playlist number
              (Utilities|Array|AddUnique (Variables|/Game/Mods/braidy08mods/HeistJukeboxRecode/HeistSoundtrackPersistentObject.HeistSoundtrackPersistentObject_C|GetPDAHeistPlaylistArray _as_heist_soundtrack_persistent_object) _array_element_2)
              (CallFunction|PrinttoModLoader (Utilities|GetClassDisplayName (Utilities|GetClass _array_element_2)))))
          (else
            (CallFunction|PrinttoModLoader "invalid class")
            (Utilities|Array|RemoveItem _pdaheistplaylistarray _array_element)))
        (else
          (CallFunction|PrinttoModLoader "invalid soft reference")
          (Utilities|Array|RemoveItem _pdaheistplaylistarray _array_element))))
    (else
      (CallFunction|PrinttoModLoader "loaded")
      (CallFunction|PrinttoModLoader (Utilities|String|Append (Utilities|String|ToString(Boolean) _output_get) (Utilities|String|ToString(Boolean) _output_get_2) (Utilities|String|ToString(Boolean) _output_get_3) (Utilities|String|ToString(Boolean) _output_get_4) (Utilities|String|ToString(Boolean) _output_get_5) (Utilities|String|ToString(Boolean) _output_get_6))))))

(fn Save
  (bind _as_heist_soundtrack_persistent_object (Variables|Default|GetAs%20Heist%20Soundtrack%20Persistent%20Object))
  (bind _savegameobject (Variables|Default|GetSaveGameObject))
  (bind _as_heist_soundtrack_persistent_object_2 (Variables|Default|GetAs%20Heist%20Soundtrack%20Persistent%20Object))
  ;[1 1 1] there has to be a better way to do this
  (bind _output_get (Variables|/Game/Mods/braidy08mods/HeistJukeboxRecode/HeistJukeboxSaveGame.HeistJukeboxSaveGame_C|SetRandomEnabled _savegameobject (Variables|/Game/Mods/braidy08mods/HeistJukeboxRecode/HeistSoundtrackPersistentObject.HeistSoundtrackPersistentObject_C|GetrandomSong _as_heist_soundtrack_persistent_object)))
  (bind _output_get_2 (Variables|/Game/Mods/braidy08mods/HeistJukeboxRecode/HeistJukeboxSaveGame.HeistJukeboxSaveGame_C|SetRandomAssaultEnabled _savegameobject (Variables|/Game/Mods/braidy08mods/HeistJukeboxRecode/HeistSoundtrackPersistentObject.HeistSoundtrackPersistentObject_C|GetassaultRandomSong _as_heist_soundtrack_persistent_object)))
  (bind _output_get_3 (Variables|/Game/Mods/braidy08mods/HeistJukeboxRecode/HeistJukeboxSaveGame.HeistJukeboxSaveGame_C|SetPlaylistEnabled _savegameobject (Variables|/Game/Mods/braidy08mods/HeistJukeboxRecode/HeistSoundtrackPersistentObject.HeistSoundtrackPersistentObject_C|GetplaylistEnabled _as_heist_soundtrack_persistent_object)))
  (bind _output_get_4 (Variables|/Game/Mods/braidy08mods/HeistJukeboxRecode/HeistJukeboxSaveGame.HeistJukeboxSaveGame_C|SetRTCStealthEnabled _savegameobject (Variables|/Game/Mods/braidy08mods/HeistJukeboxRecode/HeistSoundtrackPersistentObject.HeistSoundtrackPersistentObject_C|GetEnableRTCStealth _as_heist_soundtrack_persistent_object)))
  (bind _output_get_5 (Variables|/Game/Mods/braidy08mods/HeistJukeboxRecode/HeistJukeboxSaveGame.HeistJukeboxSaveGame_C|SetRTCFixDisabled _savegameobject (Variables|/Game/Mods/braidy08mods/HeistJukeboxRecode/HeistSoundtrackPersistentObject.HeistSoundtrackPersistentObject_C|GetdisableRTCFix _as_heist_soundtrack_persistent_object)))
  (bind _output_get_6 (Variables|/Game/Mods/braidy08mods/HeistJukeboxRecode/HeistJukeboxSaveGame.HeistJukeboxSaveGame_C|SetEnableEndlessRanTrack _savegameobject (Variables|/Game/Mods/braidy08mods/HeistJukeboxRecode/HeistSoundtrackPersistentObject.HeistSoundtrackPersistentObject_C|GetEnableEndlessRanTrack _as_heist_soundtrack_persistent_object)))
  (if (Variables|/Game/Mods/braidy08mods/HeistJukeboxRecode/HeistJukeboxSaveGame.HeistJukeboxSaveGame_C|GetPlaylistEnabled (Variables|Default|GetSaveGameObject))
    (if (>= (Utilities|Array|Length (Variables|/Game/Mods/braidy08mods/HeistJukeboxRecode/HeistSoundtrackPersistentObject.HeistSoundtrackPersistentObject_C|GetPDAHeistPlaylistArray (Variables|Default|GetAs%20Heist%20Soundtrack%20Persistent%20Object))) 1)
      (for _array_element (Variables|/Game/Mods/braidy08mods/HeistJukeboxRecode/HeistSoundtrackPersistentObject.HeistSoundtrackPersistentObject_C|GetPDAHeistPlaylistArray (Variables|Default|GetAs%20Heist%20Soundtrack%20Persistent%20Object))
        (Utilities|Array|AddUnique (Variables|/Game/Mods/braidy08mods/HeistJukeboxRecode/HeistJukeboxSaveGame.HeistJukeboxSaveGame_C|GetPDAHeistPlaylistArray (Variables|Default|GetSaveGameObject)) (Utilities|ResolveSoftReference (Utilities|GetClass _array_element))))
      (else
        (Variables|/Game/Mods/braidy08mods/HeistJukeboxRecode/HeistJukeboxSaveGame.HeistJukeboxSaveGame_C|SetPlaylistEnabled (Variables|Default|GetSaveGameObject) false)
        (Variables|/Game/Mods/braidy08mods/HeistJukeboxRecode/HeistSoundtrackPersistentObject.HeistSoundtrackPersistentObject_C|SetplaylistEnabled _as_heist_soundtrack_persistent_object_2 false)
        (Default|CallPlaylistTrackToggled _as_heist_soundtrack_persistent_object_2 false)
        (Utilities|Array|Clear (Variables|/Game/Mods/braidy08mods/HeistJukeboxRecode/HeistJukeboxSaveGame.HeistJukeboxSaveGame_C|GetPDAHeistPlaylistArray (Variables|Default|GetSaveGameObject)) :!label _label)))
    (else
      (goto _label)))
  (CallFunction|PrinttoModLoader (Utilities|String|Append (Utilities|String|ToString(Boolean) _output_get) (Utilities|String|ToString(Boolean) _output_get_2) (Utilities|String|ToString(Boolean) _output_get_3) (Utilities|String|ToString(Boolean) _output_get_4) (Utilities|String|ToString(Boolean) _output_get_5) (Utilities|String|ToString(Boolean) _output_get_6)))
  (bind _returnvalue (SaveGame|SaveGametoSlot (Variables|Default|GetSaveGameObject) "HeistJukeboxSaveGame"))
  (if _returnvalue
    (CallFunction|PrinttoModLoader "saved")
    (else
      (CallFunction|PrinttoModLoader "failed to save")))
  (return))