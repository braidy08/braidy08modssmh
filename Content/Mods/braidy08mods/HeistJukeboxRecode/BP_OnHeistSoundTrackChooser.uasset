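; Jukebox mod actor that picks and plays the soundtrack during PD3 heists, skipping tutorials.
; On BeginPlay it reads the persistent settings object, adds widgets, optionally randomizes the track, and polls until ActionPhase to play it.
; Bound heist-state changes drive assault-based rerolls, avoiding stealth-only tracks with capped retries, and timed endless rerolls at point of no return.
; An RTC fix stops that heist's nightclub music before replaying the chosen track outside stealth.
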(event Custom|OnHeistStateChanged
  (params (OldState :type EPD3HeistState%20Enum :default "Stealth") (NewState :type EPD3HeistState%20Enum :default "Stealth"))
  (bind _as_heist_soundtrack_persistent_object (Variables|Default|GetAs%20Heist%20Soundtrack%20Persistent%20Object))
  (bind _pdaheist (Variables|/Game/Mods/braidy08mods/HeistJukeboxRecode/HeistSoundtrackPersistentObject.HeistSoundtrackPersistentObject_C|GetPDAHeist _as_heist_soundtrack_persistent_object))
  (CallFunction|HeistStateChangedEvent OldState NewState)
  (if (and (Utilities|Enum|Equal(Enum) NewState "PointOfNoReturn") (Variables|/Game/Mods/braidy08mods/HeistJukeboxRecode/HeistSoundtrackPersistentObject.HeistSoundtrackPersistentObject_C|GetEnableEndlessRanTrack (Variables|Default|GetAs%20Heist%20Soundtrack%20Persistent%20Object)))
    (CallFunction|SelectRandomTrack :!label _label)
    (if (<= (Variables|Default|GetStealthReselectAttempts) 5)
      (if (Variables|/Game/Mods/HeistJukebox/PDA_HeistSoundtrack.PDA_HeistSoundtrack_C|GetStealth%20Only _pdaheist)
        (Math|Integer|IncrementInt (Variables|Default|GetStealthReselectAttempts) ; hack to prevent locking up the game
          (:%20%20
            (goto _label)))
        (else
          _))
      (else
        (Variables|Default|SetStealthReselectAttempts 0)))
    (CallFunction|PlaySong _pdaheist)
    (Utilities|FlowControl|Delay (Math|Random|RandomFloatinRange 1.2e+02 2.4e+02))
    (if (not (Utilities|Enum|Equal(Enum) (Class|SBZGameStateMachineFunctionLibrary|GetGameStateMachineState) "SM_Result"))
      (goto _label))))

(event EventBeginPlay
  (bind _persistentobject (Utilities|GetPersistentObject)
    (:Found
      (Variables|Default|SetAs%20Heist%20Soundtrack%20Persistent%20Object _persistentobject)
      (if (CallFunction|CheckSongCacheExists)
        _
        (else
          (CallFunction|LoadSongs)))
      (bind _returnvalue (Actor|GetActorOfClass "/Script/Starbreeze.PD3HeistGameState"))
      (Variables|Default|SetPD3HeistGameState _returnvalue)
      (CallFunction|PrinttoModLoader "Loaded Jukebox")
      (CallFunction|SetupinHeistWidgets)
      (CallFunction|SetupDebugStuff)
      (if (Variables|/Game/Mods/braidy08mods/HeistJukeboxRecode/HeistSoundtrackPersistentObject.HeistSoundtrackPersistentObject_C|GetJukeboxDisabled (Variables|Default|GetAs%20Heist%20Soundtrack%20Persistent%20Object))
        (CallFunction|PrinttoModLoader "Jukebox Disabled")
        (else
          (bind _validheist (CallFunction|GetCurrentHeist))
          (if _validheist
            (if (Variables|/Game/Mods/braidy08mods/HeistJukeboxRecode/HeistSoundtrackPersistentObject.HeistSoundtrackPersistentObject_C|GetrandomSong (Variables|Default|GetAs%20Heist%20Soundtrack%20Persistent%20Object))
              (CallFunction|SelectRandomTrack))
            (if (Utilities|Enum|Equal(Enum) (Class|SBZGameStateMachineFunctionLibrary|GetGameStateMachineState) "SM_ActionPhase") :!label _label
              (CallFunction|RTCFix)
              (CallFunction|PlaySong (Variables|/Game/Mods/braidy08mods/HeistJukeboxRecode/HeistSoundtrackPersistentObject.HeistSoundtrackPersistentObject_C|GetPDAHeist (Variables|Default|GetAs%20Heist%20Soundtrack%20Persistent%20Object)))
              (if (Math|Boolean|ORBoolean (Variables|/Game/Mods/braidy08mods/HeistJukeboxRecode/HeistSoundtrackPersistentObject.HeistSoundtrackPersistentObject_C|GetassaultRandomSong (Variables|Default|GetAs%20Heist%20Soundtrack%20Persistent%20Object)) (Variables|/Game/Mods/braidy08mods/HeistJukeboxRecode/HeistSoundtrackPersistentObject.HeistSoundtrackPersistentObject_C|GetplaylistEnabled (Variables|Default|GetAs%20Heist%20Soundtrack%20Persistent%20Object)) (Variables|/Game/Mods/braidy08mods/HeistJukeboxRecode/HeistSoundtrackPersistentObject.HeistSoundtrackPersistentObject_C|GetHeistIsRTC (Variables|Default|GetAs%20Heist%20Soundtrack%20Persistent%20Object)))
                (EventDispatchers|BindEventtoOnHeistStateChanged (Variables|Default|GetPD3HeistGameState) (EventDispatchers|CreateEvent :!event Custom|OnHeistStateChanged)))
              (else
                (Utilities|FlowControl|Delay 0.2)
                (goto _label)))
            (else
              (CallFunction|PrinttoModLoader "invalid heist"))))))
    (:NotFound
      (CallFunction|PrinttoModLoader "FAILED TO FIND HEIST SOUNDTRACK OBJECT"))))

(fn ConstructionScript)

(fn HeistStateChangedEvent
  (params (OldState :type EPD3HeistState%20Enum :default "Stealth") (NewState :type EPD3HeistState%20Enum :default "Stealth"))
  (CallFunction|RTCFix)
  (CallFunction|RandomSongAssaultLogic NewState))

(fn SetupDebugStuff
  (if (Variables|/Game/Mods/braidy08mods/HeistJukeboxRecode/HeistSoundtrackPersistentObject.HeistSoundtrackPersistentObject_C|Getdebug (Variables|Default|GetAs%20Heist%20Soundtrack%20Persistent%20Object))
    (bind _returnvalue (UserInterface|CreateWidget "/Game/Mods/braidy08mods/HeistJukeboxRecode/Widgets/JukeboxDebug.JukeboxDebug_C"))
    (UserInterface|Viewport|AddtoViewport _returnvalue 9999)))

(fn GetCurrentHeist
  (bind _returnvalue (Game|GetCurrentLevelName true))
  (if (Variables|/Script/Starbreeze.PD3HeistDataAsset|GetbIsTutorialLevel (Class|SBZHeistDeveloperSettings|GetHeistDatafromLevelShortName _returnvalue))
    (CallFunction|PrinttoModLoader "In Tutorial")
    (return false)
    (else
      (Variables|/Game/Mods/braidy08mods/HeistJukeboxRecode/HeistSoundtrackPersistentObject.HeistSoundtrackPersistentObject_C|SetHeistIsRTC (Variables|Default|GetAs%20Heist%20Soundtrack%20Persistent%20Object) (== (Class|SBZGameStateMachineSettings|LevelShortNametoIdx _returnvalue) 3))
      (return true))))

(fn SetupinHeistWidgets
  (bind _returnvalue (UserInterface|CreateWidget "/Game/Mods/braidy08mods/HeistJukeboxRecode/Widgets/JukeboxCurrentSong.JukeboxCurrentSong_C"))
  (UserInterface|Viewport|AddtoViewport _returnvalue 9999))

(fn RandomSongAssaultLogic
  (params (Selection :type EPD3HeistState%20Enum :default "Stealth"))
  (bind _as_heist_soundtrack_persistent_object (Variables|Default|GetAs%20Heist%20Soundtrack%20Persistent%20Object))
  (bind _as_heist_soundtrack_persistent_object_2 (Variables|Default|GetAs%20Heist%20Soundtrack%20Persistent%20Object))
  (bind _as_heist_soundtrack_persistent_object_3 (Variables|Default|GetAs%20Heist%20Soundtrack%20Persistent%20Object))
  (bind _pdaheist (Variables|/Game/Mods/braidy08mods/HeistJukeboxRecode/HeistSoundtrackPersistentObject.HeistSoundtrackPersistentObject_C|GetPDAHeist _as_heist_soundtrack_persistent_object_2))
  (bind _pdaheist_2 (Variables|/Game/Mods/braidy08mods/HeistJukeboxRecode/HeistSoundtrackPersistentObject.HeistSoundtrackPersistentObject_C|GetPDAHeist _as_heist_soundtrack_persistent_object_3))
  (bind _stealth_only (Variables|/Game/Mods/HeistJukebox/PDA_HeistSoundtrack.PDA_HeistSoundtrack_C|GetStealth%20Only _pdaheist))
  (if (or (Variables|/Game/Mods/braidy08mods/HeistJukeboxRecode/HeistSoundtrackPersistentObject.HeistSoundtrackPersistentObject_C|GetassaultRandomSong _as_heist_soundtrack_persistent_object) (Variables|/Game/Mods/braidy08mods/HeistJukeboxRecode/HeistSoundtrackPersistentObject.HeistSoundtrackPersistentObject_C|GetplaylistEnabled _as_heist_soundtrack_persistent_object))
    (switch Utilities|FlowControl|Switch|SwitchonEPD3HeistState Selection
      (:Alarm
        (if _stealth_only :!label _label
          (CallFunction|SelectRandomTrack :!label _label_2)
          (if (<= (Variables|Default|GetStealthReselectAttempts) 6)
            (if (Variables|/Game/Mods/HeistJukebox/PDA_HeistSoundtrack.PDA_HeistSoundtrack_C|GetStealth%20Only _pdaheist_2)
              (Math|Integer|IncrementInt (Variables|Default|GetStealthReselectAttempts) ; hack to prevent locking up the game
                (:%20%20
                  (goto _label_2)))
              (else
                _))
            (else
              (Variables|Default|SetStealthReselectAttempts 0)))
          (CallFunction|PlaySong _pdaheist_2)
          (CallFunction|PrinttoModLoader (Utilities|String|ToString(Boolean) (Variables|Default|GetAssaultActive)))))
      (:Anticipation
        (goto _label))
      (:Assault
        (if _stealth_only
          (goto _label_2)
          (elif (not (Variables|Default|GetAssaultActive))
            (Variables|Default|SetAssaultActive true))))
      (:Control
        (if _stealth_only
          (goto _label_2)
          (elif (Variables|Default|GetAssaultActive)
            (Variables|Default|SetAssaultActive false)
            (goto _label_2)))))))

(fn RTCFix
  (bind _returnvalue (Class|SBZMusicManager|GetMusicManager))
  (bind _as_heist_soundtrack_persistent_object (Variables|Default|GetAs%20Heist%20Soundtrack%20Persistent%20Object))
  (bind _pd3heistgamestate (Variables|Default|GetPD3HeistGameState))
  (bind _returnvalue_2 (Class|PD3HeistGameState|GetCurrentHeistState _pd3heistgamestate))
  (bind _returnvalue_3 (Utilities|Enum|Equal(Enum) _returnvalue_2 "Search"))
  (bind _returnvalue_4 (Utilities|Enum|Equal(Enum) _returnvalue_2 "Stealth"))
  (bind _returnvalue_5 (Math|Boolean|NORBoolean _returnvalue_4 _returnvalue_3))
  (if (Math|Boolean|ANDBoolean (not (Variables|Default|GetRTC_FixActive)) (not (Variables|/Game/Mods/braidy08mods/HeistJukeboxRecode/HeistSoundtrackPersistentObject.HeistSoundtrackPersistentObject_C|GetdisableRTCFix _as_heist_soundtrack_persistent_object)) (Variables|/Game/Mods/braidy08mods/HeistJukeboxRecode/HeistSoundtrackPersistentObject.HeistSoundtrackPersistentObject_C|GetHeistIsRTC _as_heist_soundtrack_persistent_object))
    (if (Variables|/Game/Mods/braidy08mods/HeistJukeboxRecode/HeistSoundtrackPersistentObject.HeistSoundtrackPersistentObject_C|GetEnableRTCStealth _as_heist_soundtrack_persistent_object)
      (Variables|Default|SetRTC_FixActive true)
      (Class|SBZMusicManager|StopMusic _returnvalue :!label _label)
      (Class|SBZMusicManager|PlayMusic _returnvalue "/Game/WwiseAudio/Events/Music/System/Music_Stop_Nightclub_Diagetic.Music_Stop_Nightclub_Diagetic" false)
      (if _returnvalue_5
        (CallFunction|PlaySong (Variables|/Game/Mods/braidy08mods/HeistJukeboxRecode/HeistSoundtrackPersistentObject.HeistSoundtrackPersistentObject_C|GetPDAHeist (Variables|Default|GetAs%20Heist%20Soundtrack%20Persistent%20Object))))
      (elif _returnvalue_5
        (Variables|Default|SetRTC_FixActive true)
        (goto _label)))))