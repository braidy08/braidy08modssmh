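; Escort van variant for a sabotage heist, handling escort-zone visuals and engine audio on non-dedicated-server instances.
; Escort mode toggles a Niagara zone effect, which is enlarged when the preplanning size upgrade applies.
; Escorting player count plays or reverses a timeline meant to drive the effect, alongside Wwise events and engine RPM.
; Spline movement start plays engine audio once, cut after a fixed delay; a helper opens the rear doors.
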(event OnStarted(SplineFollowingComponent)
  (bind _ak (Variables|Default|GetAk))
  (if (not (Networking|IsDedicatedServer))
    (Utilities|FlowControl|DoOnce false
      (:Completed
        (Class|AkGameObject|PostAkEvent (Variables|Default|GetAk) "/Game/WwiseAudio/Events/Vehicles/Veh_Truck_Generic/Truck_A_Engine.Truck_A_Engine")
        (Utilities|FlowControl|DoOnce false
          (:Completed
            (Utilities|FlowControl|Delay 34.0)
            (Class|AkGameObject|PostAkEvent _ak "/Game/WwiseAudio/Events/Vehicles/Veh_Truck_Generic/Truck_A_Engine_Off.Truck_A_Engine_Off")
            (Class|AkGameObject|SetRTPCValue _ak "/Game/WwiseAudio/Game_Parameters/Default_Work_Unit/Vehicles/Engine_RPM.Engine_RPM" 0.0)))))))

(event EventOnEscortModeChanged
  (params (bEnabled :type Boolean) (bDoCosmetics :type Boolean))
  (bind _niagara_escort (Variables|Default|GetNiagara%20Escort))
  (|CallParentFunction bEnabled bDoCosmetics)
  (if (not (Networking|IsDedicatedServer))
    (if bEnabled
      (Components|Activation|Activate _niagara_escort false)
      (else
        (Components|Activation|Deactivate _niagara_escort)))))

(event EventOnEscortSizePreplanningApplied
  (|CallParentFunction)
  (if (not (Networking|IsDedicatedServer))
    (Transformation|SetWorldScale3D (Variables|Default|GetNiagara%20Escort) "7.500000,7.500000,1.000000")))

(event EventOnPlayersinEscortChanged
  (params (PlayersEscorting :type Integer))
  (bind _ak (Variables|Default|GetAk))
  (bind _escortzonetimeline (Variables|Default|GetEscortZoneTimeline))
  (|CallParentFunction PlayersEscorting)
  (if (not (Networking|IsDedicatedServer))
    (if (> PlayersEscorting 0)
      (Class|AkGameObject|PostAkEvent _ak "/Game/WwiseAudio/Events/Vehicles/Veh_Truck_Generic/Truck_A_Circle_Activate.Truck_A_Circle_Activate")
      (Class|AkGameObject|SetRTPCValue _ak "/Game/WwiseAudio/Game_Parameters/Default_Work_Unit/Vehicles/Engine_RPM.Engine_RPM" 1e+02)
      (Components|Timeline|PlayfromStart _escortzonetimeline)
      (else
        (Components|Timeline|ReversefromEnd _escortzonetimeline)))))

(fn ConstructionScript)

(fn OpenRearDoors
  (Class|SBZSabotagableVehicle|SetRearDoorsState "Opened"))