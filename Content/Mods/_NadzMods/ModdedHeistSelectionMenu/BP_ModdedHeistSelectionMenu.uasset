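; Actor that drives a modded heist selection menu, listing custom heists and launching them as solo games.
; On widget spawn, it filters all heist data, dropping prototype tutorial maps and, in shipping builds, base-game levels.
; It builds CrimeNet text buttons mapped to their heist data.
; Hovering shows the description and best stealth/loud times per difficulty, while selecting requests a solo game through the game state machine.
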(event Custom|OnHeistButtonSelected
  (params (Button :type SBZ%20Menu%20Button%20Object%20Reference))
  (Widget|SetVisibility (Variables|/Game/Mods/_NadzMods/ModdedHeistSelectionMenu/UI/WBP_UI_ModdedHeists_HeistSelection.WBP_UI_ModdedHeists_HeistSelection_C|GetOverlay_PanelSpace (Variables|Default|GetModdedHeistsMenu)) "Collapsed")
  (bind _aswbp_ui_crime_net_text_button (Utilities|Casting|CastToWBP_UI_CrimeNet_TextButton Button))
  (Class|SBZOnlineFunctionLibrary|SetSoloGameEnabled)
  (Class|SBZGameStateMachine|RequestSoloGame (Class|SBZGameStateMachineFunctionLibrary|GetGameStateMachine) (Class|SBZGameStateMachineSettings|LevelPathtoIdx (.LevelPath (Utilities|Struct|BreakSBZHeistDataLevelPair (.Value (Utilities|Map|Find (Variables|Default|GetHeistDataButtonsMap) _aswbp_ui_crime_net_text_button))))) (Variables|/Game/Mods/_NadzMods/ModdedHeistSelectionMenu/UI/WBP_UI_ModdedHeists_HeistSelection.WBP_UI_ModdedHeists_HeistSelection_C|GetCurrentDifficultyIndex (Variables|Default|GetModdedHeistsMenu)) false))

(event Custom|OnButtonHover
  (params (Button :type SBZ%20Menu%20Button%20Object%20Reference) (bIsEnabled :type Boolean))
  (bind _aswbp_ui_crime_net_text_button (Utilities|Casting|CastToWBP_UI_CrimeNet_TextButton Button))
  (Variables|Default|SetSelectedButton _aswbp_ui_crime_net_text_button)
  (Variables|/Game/Mods/_NadzMods/ModdedHeistSelectionMenu/UI/WBP_UI_ModdedHeists_HeistSelection.WBP_UI_ModdedHeists_HeistSelection_C|SetActiveHeistButton (Variables|Default|GetModdedHeistsMenu) (Variables|Default|GetSelectedButton))
  (CallFunction|SetSelectedHeistInfo (Variables|Default|GetSelectedButton)))

(event Custom|SpawnWidget
  (params (HeistMenu :type WBP%20UI%20Modded%20Heists%20Heist%20Selection%20Object%20Reference))
  (bind _output_get (Variables|Default|SetModdedHeistsMenu HeistMenu))
  (Variables|/Game/Mods/_NadzMods/ModdedHeistSelectionMenu/UI/WBP_UI_ModdedHeists_HeistSelection.WBP_UI_ModdedHeists_HeistSelection_C|SetModdedHeistSelectorActor _output_get self)
  (UserInterface|Viewport|AddtoViewport _output_get 0)
  (Widget|SetVisibility _output_get "Collapsed")
  (CallFunction|GetHeistInfo)
  (CallFunction|MakeModdedHeistButtons)
  (bind _keys (Utilities|Map|Keys (Variables|Default|GetHeistDataButtonsMap)))
  (for (_array_element _array_index) _keys
    (Widget|Panel|AddChild (Variables|/Game/Mods/_NadzMods/ModdedHeistSelectionMenu/UI/WBP_UI_ModdedHeists_HeistSelection.WBP_UI_ModdedHeists_HeistSelection_C|GetScrollBox_LevelList (Variables|Default|GetModdedHeistsMenu)) _array_element)
    (if (== _array_index 0)
      (bind _output_get_2 (Variables|Default|SetSelectedButton _array_element))
      (CallFunction|SetSelectedHeistInfo _output_get_2))))

(event EventBeginPlay)

(fn ConstructionScript)

(fn GetHeistInfo
  (Utilities|FlowControl|Sequence
    (:then_0
      (for _array_element (Class|SBZGameStateMachineSettings|GetHeistCollections)
        (for _array_element_2 (.LevelPaths (Utilities|Struct|BreakSBZHeistCollection _array_element))
          (Utilities|Array|AddUnique (Variables|Default|GetGameHeistsLevelPaths) _array_element_2)))
      (for _array_element_3 (Class|SBZGameStateMachineSettings|GetLevelsTutorial)
        (Utilities|Array|AddUnique (Variables|Default|GetGameHeistsLevelPaths) _array_element_3)))
    (:then_1
      (for _array_element_4 (Class|SBZHeistDeveloperSettings|GetAllHeistData)
        (if (not (or (and (Utilities|Array|ContainsItem (Variables|Default|GetGameHeistsLevelPaths) (.LevelPath (Utilities|Struct|BreakSBZHeistDataLevelPair _array_element_4))) (Class|SBZOnlineFunctionLibrary|IsShippingBuild)) (Utilities|String|Contains (Utilities|BreakSoftObjectPath (.LevelPath (Utilities|Struct|BreakSBZHeistDataLevelPair _array_element_4))) "/Game/Prototype/Maps/Tutorial")))
          (Utilities|Array|AddUnique (Variables|Default|GetModdedHeistsArray) _array_element_4))))))

(fn MakeModdedHeistButtons
  (Utilities|Map|Clear (Variables|Default|GetHeistDataButtonsMap))
  (Widget|Panel|ClearChildren (Variables|/Game/Mods/_NadzMods/ModdedHeistSelectionMenu/UI/WBP_UI_ModdedHeists_HeistSelection.WBP_UI_ModdedHeists_HeistSelection_C|GetScrollBox_LevelList (Variables|Default|GetModdedHeistsMenu)))
  (for _array_element (Variables|Default|GetModdedHeistsArray)
    (bind _returnvalue (UserInterface|CreateWidget "/Game/UI/Widgets/Menus/Buttons/WBP_UI_CrimeNet_TextButton.WBP_UI_CrimeNet_TextButton_C"))
    (Default|SetButtonText _returnvalue (Variables|/Script/Starbreeze.PD3HeistDataAsset|GetHeistDisplayName (.HeistData (Utilities|Struct|BreakSBZHeistDataLevelPair _array_element))))
    ;[0 0 0] Possibly add best time here
    (Default|SetTextDescription _returnvalue)
    (if (Utilities|IsValidSoftObjectReference (Variables|/Script/Starbreeze.PD3HeistDataAsset|GetHeistBannerImage (.HeistData (Utilities|Struct|BreakSBZHeistDataLevelPair _array_element))))
      (bind _returnvalue_2 (Utilities|LoadAssetBlocking (Variables|/Script/Starbreeze.PD3HeistDataAsset|GetHeistBannerImage (.HeistData (Utilities|Struct|BreakSBZHeistDataLevelPair _array_element)))))
      (bind _aspaper_sprite (Utilities|Casting|CastToPaperSprite _returnvalue_2))
      (Variables|/Game/UI/Widgets/Menus/Buttons/WBP_UI_CrimeNet_TextButton.WBP_UI_CrimeNet_TextButton_C|SetPaperSprite_Image_Buttons _returnvalue _aspaper_sprite)
      (else
        (Variables|/Game/UI/Widgets/Menus/Buttons/WBP_UI_CrimeNet_TextButton.WBP_UI_CrimeNet_TextButton_C|SetPaperSprite_Image_Buttons _returnvalue "/Game/Mods/_NadzMods/ModdedHeistSelectionMenu/UI/Textures/SS_UI_Placeholder_Banner_Sprite.SS_UI_Placeholder_Banner_Sprite")))
    (Layout|BorderSlot|SetPadding _returnvalue (Utilities|Struct|MakeMargin 0.0 0.0 0.0 5.0) :!class /Script/UMG.UserWidget)
    (EventDispatchers|BindEventtoOnButtonSelected _returnvalue (EventDispatchers|CreateEvent :!event Custom|OnHeistButtonSelected))
    (EventDispatchers|BindEventtoOnButtonFocusedChanged _returnvalue (EventDispatchers|CreateEvent :!event Custom|OnButtonHover))
    (Utilities|Map|Add (Variables|Default|GetHeistDataButtonsMap) _returnvalue _array_element)))

(fn SetSelectedHeistInfo
  (params (SelectedButton :type WBP%20UI%20Crime%20Net%20Text%20Button%20Object%20Reference))
  (bind _heistdatabuttonsmap (Variables|Default|GetHeistDataButtonsMap))
  (bind _value (Utilities|Map|Find _heistdatabuttonsmap SelectedButton))
  (bind (_heistdata _levelpath) (Utilities|Struct|BreakSBZHeistDataLevelPair _value))
  (|SetStealthTimeTextToArray)
  (|SetLoudTimeTextToArray)
  (Utilities|Array|Clear (Variables|Default|GetStealthTimes))
  (Utilities|Array|Clear (Variables|Default|GetLoudTimes))
  (Rendering|Components|TextRender|SetText (Variables|/Game/Mods/_NadzMods/ModdedHeistSelectionMenu/UI/WBP_UI_ModdedHeists_HeistSelection.WBP_UI_ModdedHeists_HeistSelection_C|GetText_Desc_LevelDescription (Variables|Default|GetModdedHeistsMenu)) (Variables|/Script/Starbreeze.PD3HeistDataAsset|GetHeistDescription _heistdata))
  (for _array_element (Class|SBZPlayerStatisticsManager|GetHeistBestTimes (Class|SBZPlayerStatisticsManager|GetPlayerStatisticsManager) _levelpath)
    (Utilities|Array|Add (Variables|Default|GetStealthTimes) (Utilities|String|ToString(Float) (.StealthTime (Utilities|Struct|BreakSBZLevelTimesStruct _array_element))))
    (Utilities|Array|Add (Variables|Default|GetLoudTimes) (Utilities|String|ToString(Float) (.LoudTime (Utilities|Struct|BreakSBZLevelTimesStruct _array_element))))
    (for (_array_element_2 _array_index) (LocalVariables|GetStealthTimeText)
      (if (== (Math|Conversions|ToFloat(Integer) (Utilities|Array|Get(acopy) (Variables|Default|GetStealthTimes) _array_index)) -1.0)
        (Rendering|Components|TextRender|SetText _array_element_2 "N/A")
        (else
          (bind _returnvalue (Class|SBZUIStatics|FormatInttoTimerText (Math|Float|Truncate (Math|Conversions|ToFloat(Integer) (Utilities|Array|Get(acopy) (Variables|Default|GetStealthTimes) _array_index))) false))
          (Rendering|Components|TextRender|SetText _array_element_2 _returnvalue)))
      (for (_array_element_3 _array_index_2) (LocalVariables|GetLoudTimeText)
        (if (== (Math|Conversions|ToFloat(Integer) (Utilities|Array|Get(acopy) (Variables|Default|GetLoudTimes) _array_index_2)) -1.0)
          (Rendering|Components|TextRender|SetText _array_element_3 "N/A")
          (else
            (bind _returnvalue_2 (Class|SBZUIStatics|FormatInttoTimerText (Math|Float|Truncate (Math|Conversions|ToFloat(Integer) (Utilities|Array|Get(acopy) (Variables|Default|GetLoudTimes) _array_index_2))) false))
            (Rendering|Components|TextRender|SetText _array_element_3 _returnvalue_2)))))))

(fn GetMainMenuCrimenet)