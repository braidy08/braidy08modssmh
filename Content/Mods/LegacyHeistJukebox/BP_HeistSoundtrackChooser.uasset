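; Heist jukebox mod actor that lets players pick heist music in the preplanning lobby.
; It scans the mod's Music folder for soundtrack data assets and shares them through a persistent mod object.
; On lobby entry it selects the heist's default track from a data table and spawns a selector widget with arrows, track menu and option toggles.
; Random-song and RTC options persist in a save slot, while playlists and disabling reset each lobby.
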(event Custom|EventOnPreMatchAsyncLoadingDone_0
  ;[1 0 0] UNUSED
)

(event Custom|EventOnRightButtonClicked_0
  (bind _as_heist_soundtrack_persistent_object (Variables|Default|GetAs%20Heist%20Soundtrack%20Persistent%20Object))
  ;[0.3733 0.8389 1] Handle changing soundtrack from button click
  (bind _result (Math|Integer|IncrementInt (Variables|Default|GetIndex))
    (:%20%20
      (if (== _result (Utilities|Array|Length (Variables|Default|GetPDAHeistSoundtrackarray)))
        (Variables|Default|SetIndex 0))
      (bind _pdaheistsoundtrack (CallFunction|GetCurrentPDA (Variables|Default|GetIndex)))
      (Default|SetWidgetText (Variables|Default|GetSoundtrack%20Selector%20Widget) (Variables|/Game/Mods/HeistJukebox/PDA_HeistSoundtrack.PDA_HeistSoundtrack_C|GetName _pdaheistsoundtrack))
      (Variables|/Game/Mods/braidy08mods/HeistJukeboxRecode/HeistSoundtrackPersistentObject.HeistSoundtrackPersistentObject_C|SetPDAHeist _as_heist_soundtrack_persistent_object _pdaheistsoundtrack)
      (Variables|/Game/Mods/braidy08mods/HeistJukeboxRecode/HeistSoundtrackPersistentObject.HeistSoundtrackPersistentObject_C|SetIndex _as_heist_soundtrack_persistent_object (Variables|Default|GetIndex))
      (Utilities|Debugtextprint))))

(event Custom|OnStateMachineEnteredLobby_Event_0
  (bind _as_heist_soundtrack_persistent_object (Variables|Default|GetAs%20Heist%20Soundtrack%20Persistent%20Object))
  ;[0.5462 1 0.5603] Spawn Soundtrack selector widget once preplanning lobby is loaded
  (Variables|/Game/Mods/braidy08mods/HeistJukeboxRecode/HeistSoundtrackPersistentObject.HeistSoundtrackPersistentObject_C|SetJukeboxDisabled (Variables|Default|GetAs%20Heist%20Soundtrack%20Persistent%20Object) false)
  (CallFunction|SetDefaultPDAPerHeist)
  (Variables|/Game/Mods/braidy08mods/HeistJukeboxRecode/HeistSoundtrackPersistentObject.HeistSoundtrackPersistentObject_C|SetplaylistEnabled _as_heist_soundtrack_persistent_object false)
  (Utilities|Array|Clear (Variables|/Game/Mods/braidy08mods/HeistJukeboxRecode/HeistSoundtrackPersistentObject.HeistSoundtrackPersistentObject_C|GetPDAHeistPlaylistArray _as_heist_soundtrack_persistent_object))
  (bind _returnvalue (UserInterface|CreateWidget "/Game/Mods/LegacyHeistJukebox/WBP_SoundtrackSelector.WBP_SoundtrackSelector_C"))
  (bind _output_get (Variables|Default|SetSoundtrack%20Selector%20Widget _returnvalue))
  (bind _pdaheistsoundtrack (CallFunction|GetCurrentPDA (Variables|Default|GetIndex)))
  (Default|SetWidgetText _output_get (Variables|/Game/Mods/HeistJukebox/PDA_HeistSoundtrack.PDA_HeistSoundtrack_C|GetName _pdaheistsoundtrack))
  (UserInterface|Viewport|AddtoViewport (Variables|Default|GetSoundtrack%20Selector%20Widget) 9999)
  (CallFunction|LoadSave)
  (EventDispatchers|BindEventtoOnClicked (Variables|/Game/Mods/LegacyHeistJukebox/WBP_SoundtrackSelector.WBP_SoundtrackSelector_C|GetButton_LeftArrow (Variables|Default|GetSoundtrack%20Selector%20Widget)) (EventDispatchers|CreateEvent :!event Custom|EventOnLeftButtonClicked_0))
  (EventDispatchers|BindEventtoOnClicked (Variables|/Game/Mods/LegacyHeistJukebox/WBP_SoundtrackSelector.WBP_SoundtrackSelector_C|GetButton_RightArrow (Variables|Default|GetSoundtrack%20Selector%20Widget)) (EventDispatchers|CreateEvent :!event Custom|EventOnRightButtonClicked_0))
  (EventDispatchers|BindEventtoOnClicked (Variables|/Game/Mods/LegacyHeistJukebox/WBP_SoundtrackSelector.WBP_SoundtrackSelector_C|GetButton_SongMenu (Variables|Default|GetSoundtrack%20Selector%20Widget)) (EventDispatchers|CreateEvent :!event Custom|EventOnSongMenuButtonClicked_0))
  (EventDispatchers|BindEventtoOnButtonSelected (Variables|/Game/Mods/LegacyHeistJukebox/WBP_SoundtrackSelector.WBP_SoundtrackSelector_C|Getrandomsong (Variables|Default|GetSoundtrack%20Selector%20Widget)) (EventDispatchers|CreateEvent :!event Custom|EventOnRandomButtonClicked_0))
  (EventDispatchers|BindEventtoOnButtonSelected (Variables|/Game/Mods/LegacyHeistJukebox/WBP_SoundtrackSelector.WBP_SoundtrackSelector_C|Getrandomsongass (Variables|Default|GetSoundtrack%20Selector%20Widget)) (EventDispatchers|CreateEvent :!event Custom|EventOnAssaultRandomButtonClicked_0))
  (EventDispatchers|BindEventtoOnButtonSelected (Variables|/Game/Mods/LegacyHeistJukebox/WBP_SoundtrackSelector.WBP_SoundtrackSelector_C|Getenablertcstealth (Variables|Default|GetSoundtrack%20Selector%20Widget)) (EventDispatchers|CreateEvent :!event Custom|EventOnUIEnableButtonClicked_0))
  (EventDispatchers|BindEventtoOnButtonSelected (Variables|/Game/Mods/LegacyHeistJukebox/WBP_SoundtrackSelector.WBP_SoundtrackSelector_C|Getclearplaylist (Variables|Default|GetSoundtrack%20Selector%20Widget)) (EventDispatchers|CreateEvent :!event Custom|EventOnClearPlaylistButtonClicked_0))
  (EventDispatchers|BindEventtoOnButtonSelected (Variables|/Game/Mods/LegacyHeistJukebox/WBP_SoundtrackSelector.WBP_SoundtrackSelector_C|Getdisablertcfix (Variables|Default|GetSoundtrack%20Selector%20Widget)) (EventDispatchers|CreateEvent :!event Custom|EventOnDisableRTCFixButtonClicked_0))
  (EventDispatchers|BindEventtoOnButtonSelected (Variables|/Game/Mods/LegacyHeistJukebox/WBP_SoundtrackSelector.WBP_SoundtrackSelector_C|Getdisablemod (Variables|Default|GetSoundtrack%20Selector%20Widget)) (EventDispatchers|CreateEvent :!event Custom|EventOnDisableButtonClicked_0)))

(event Custom|heisttrackinput
  (params (Index :type Integer) (PDAHeist :type PDA%20Heist%20Soundtrack%20Object%20Reference))
  (bind _as_heist_soundtrack_persistent_object (Variables|Default|GetAs%20Heist%20Soundtrack%20Persistent%20Object))
  ;[1 0.8976 0] whatever this abomination is
  (bind _output_get (Variables|Default|SetIndex Index))
  (bind _pdaheistsoundtrack (CallFunction|GetCurrentPDA Index))
  (Default|SetWidgetText (Variables|Default|GetSoundtrack%20Selector%20Widget) (Variables|/Game/Mods/HeistJukebox/PDA_HeistSoundtrack.PDA_HeistSoundtrack_C|GetName _pdaheistsoundtrack))
  (Variables|/Game/Mods/braidy08mods/HeistJukeboxRecode/HeistSoundtrackPersistentObject.HeistSoundtrackPersistentObject_C|SetPDAHeist _as_heist_soundtrack_persistent_object _pdaheistsoundtrack)
  (Variables|/Game/Mods/braidy08mods/HeistJukeboxRecode/HeistSoundtrackPersistentObject.HeistSoundtrackPersistentObject_C|SetIndex _as_heist_soundtrack_persistent_object _output_get)
  (Utilities|Debugtextprint))

(event Custom|EventOnDisableButtonClicked_0
  (params (Button :type SBZ%20Menu%20Button%20Object%20Reference))
  (bind _as_heist_soundtrack_persistent_object (Variables|Default|GetAs%20Heist%20Soundtrack%20Persistent%20Object))
  ;[0.2041 0 1] button clicking
  (Variables|/Game/Mods/braidy08mods/HeistJukeboxRecode/HeistSoundtrackPersistentObject.HeistSoundtrackPersistentObject_C|SetJukeboxDisabled _as_heist_soundtrack_persistent_object (select (Variables|/Game/Mods/braidy08mods/HeistJukeboxRecode/HeistSoundtrackPersistentObject.HeistSoundtrackPersistentObject_C|GetJukeboxDisabled _as_heist_soundtrack_persistent_object) false true)))

(event Custom|OnStateMachineExitedLobby_Event_0
  (CallFunction|SetupPreLobby))

(event Custom|EventOnLeftButtonClicked_0
  (bind _as_heist_soundtrack_persistent_object (Variables|Default|GetAs%20Heist%20Soundtrack%20Persistent%20Object))
  ;[0.3733 0.8389 1] Handle changing soundtrack from button click
  (bind _result (Math|Integer|DecrementInt (Variables|Default|GetIndex))
    (:%20%20
      (if (== _result -1)
        (Variables|Default|SetIndex (Utilities|Array|LastIndex (Variables|Default|GetPDAHeistSoundtrackarray))))
      (bind _pdaheistsoundtrack (CallFunction|GetCurrentPDA (Variables|Default|GetIndex)))
      (Default|SetWidgetText (Variables|Default|GetSoundtrack%20Selector%20Widget) (Variables|/Game/Mods/HeistJukebox/PDA_HeistSoundtrack.PDA_HeistSoundtrack_C|GetName _pdaheistsoundtrack))
      (Variables|/Game/Mods/braidy08mods/HeistJukeboxRecode/HeistSoundtrackPersistentObject.HeistSoundtrackPersistentObject_C|SetPDAHeist _as_heist_soundtrack_persistent_object _pdaheistsoundtrack)
      (Variables|/Game/Mods/braidy08mods/HeistJukeboxRecode/HeistSoundtrackPersistentObject.HeistSoundtrackPersistentObject_C|SetIndex _as_heist_soundtrack_persistent_object (Variables|Default|GetIndex))
      (Utilities|Debugtextprint))))

(event Custom|EventOnDisableRTCFixButtonClicked_0
  (params (Button :type SBZ%20Menu%20Button%20Object%20Reference))
  (bind _as_heist_soundtrack_persistent_object (Variables|Default|GetAs%20Heist%20Soundtrack%20Persistent%20Object))
  ;[0.2041 0 1] button clicking
  (Variables|/Game/Mods/braidy08mods/HeistJukeboxRecode/HeistSoundtrackPersistentObject.HeistSoundtrackPersistentObject_C|SetdisableRTCFix _as_heist_soundtrack_persistent_object (select (Variables|/Game/Mods/braidy08mods/HeistJukeboxRecode/HeistSoundtrackPersistentObject.HeistSoundtrackPersistentObject_C|GetdisableRTCFix _as_heist_soundtrack_persistent_object) false true))
  (CallFunction|SaveSave))

(event Custom|EventOnSongMenuButtonClicked_0
  (bind _heisttracksarrayt (Variables|Default|GetHeistTracksArrayT))
  (bind _soundtrack_selector_widget (Variables|Default|GetSoundtrack%20Selector%20Widget))
  (bind _wbp_searchwidget (Variables|/Game/Mods/LegacyHeistJukebox/WBP_SoundtrackSelector.WBP_SoundtrackSelector_C|GetWBP_SearchWidget _soundtrack_selector_widget))
  ;[1 0.8976 0] whatever this abomination is
  (if (not (Variables|/Game/Mods/LegacyHeistJukebox/WBP_SoundtrackSelector.WBP_SoundtrackSelector_C|GethasHTbeencreated _soundtrack_selector_widget))
    (Variables|/Game/Mods/LegacyHeistJukebox/WBP_SoundtrackSelector.WBP_SoundtrackSelector_C|SethasHTbeencreated _soundtrack_selector_widget true)
    (Utilities|Array|Clear _heisttracksarrayt)
    (for (_array_element _array_index) (Variables|Default|GetPDAHeistSoundtrackarray)
      (bind _returnvalue (UserInterface|CreateWidget "/Game/Mods/LegacyHeistJukebox/WBP_HeistTrack.WBP_HeistTrack_C"))
      (Variables|/Game/Mods/LegacyHeistJukebox/WBP_HeistTrack.WBP_HeistTrack_C|Setisinheist _returnvalue false)
      (Rendering|Components|TextRender|SetText (Variables|/Game/Mods/LegacyHeistJukebox/WBP_HeistTrack.WBP_HeistTrack_C|Gettrackname _returnvalue) (Variables|/Game/Mods/HeistJukebox/PDA_HeistSoundtrack.PDA_HeistSoundtrack_C|GetName _array_element))
      (Variables|/Game/Mods/LegacyHeistJukebox/WBP_HeistTrack.WBP_HeistTrack_C|SetSoundtrack _returnvalue _array_element)
      (Variables|/Game/Mods/LegacyHeistJukebox/WBP_HeistTrack.WBP_HeistTrack_C|SetHTIndex _returnvalue _array_index)
      (Class|VerticalBox|AddChildtoVerticalBox (Variables|/Game/Mods/LegacyHeistJukebox/WBP_SearchWidget.WBP_SearchWidget_C|Getverticalboxgaming _wbp_searchwidget) _returnvalue)
      (Utilities|Array|Add _heisttracksarrayt _returnvalue))
    (Utilities|Array|AppendArray (Variables|/Game/Mods/LegacyHeistJukebox/WBP_SearchWidget.WBP_SearchWidget_C|GetHeistTrackArraySearch _wbp_searchwidget) _heisttracksarrayt)))

(event Custom|EventOnRandomButtonClicked_0
  (params (Button :type SBZ%20Menu%20Button%20Object%20Reference))
  (bind _as_heist_soundtrack_persistent_object (Variables|Default|GetAs%20Heist%20Soundtrack%20Persistent%20Object))
  ;[0.2041 0 1] button clicking
  (Variables|/Game/Mods/braidy08mods/HeistJukeboxRecode/HeistSoundtrackPersistentObject.HeistSoundtrackPersistentObject_C|SetrandomSong _as_heist_soundtrack_persistent_object (select (Variables|/Game/Mods/braidy08mods/HeistJukeboxRecode/HeistSoundtrackPersistentObject.HeistSoundtrackPersistentObject_C|GetrandomSong _as_heist_soundtrack_persistent_object) false true))
  (CallFunction|SaveSave))

(event Custom|EventOnAssaultRandomButtonClicked_0
  (params (Button :type SBZ%20Menu%20Button%20Object%20Reference))
  (bind _as_heist_soundtrack_persistent_object (Variables|Default|GetAs%20Heist%20Soundtrack%20Persistent%20Object))
  ;[0.2041 0 1] button clicking
  (Variables|/Game/Mods/braidy08mods/HeistJukeboxRecode/HeistSoundtrackPersistentObject.HeistSoundtrackPersistentObject_C|SetassaultRandomSong _as_heist_soundtrack_persistent_object (select (Variables|/Game/Mods/braidy08mods/HeistJukeboxRecode/HeistSoundtrackPersistentObject.HeistSoundtrackPersistentObject_C|GetassaultRandomSong _as_heist_soundtrack_persistent_object) false true))
  (CallFunction|SaveSave))

(event Custom|OnClicked_Event_0
  ;[1 0 0] UNUSED
)

(event Custom|EventOnUIEnableButtonClicked_0
  (params (Button :type SBZ%20Menu%20Button%20Object%20Reference))
  (bind _as_heist_soundtrack_persistent_object (Variables|Default|GetAs%20Heist%20Soundtrack%20Persistent%20Object))
  ;[0.2041 0 1] button clicking
  (Variables|/Game/Mods/braidy08mods/HeistJukeboxRecode/HeistSoundtrackPersistentObject.HeistSoundtrackPersistentObject_C|SetEnableRTCStealth _as_heist_soundtrack_persistent_object (select (Variables|/Game/Mods/braidy08mods/HeistJukeboxRecode/HeistSoundtrackPersistentObject.HeistSoundtrackPersistentObject_C|GetEnableRTCStealth _as_heist_soundtrack_persistent_object) false true))
  (CallFunction|SaveSave))

(event Custom|EventOnClearPlaylistButtonClicked_0
  (params (Button :type SBZ%20Menu%20Button%20Object%20Reference))
  ;[0.2041 0 1] button clicking
  (Default|Debugtextupdate (Variables|Default|GetSoundtrack%20Selector%20Widget))
  (for _array_element (Variables|Default|GetHeistTracksArrayT)
    (Default|Resetplaylist _array_element)))

(event EventBeginPlay
  ;[1 0.4324 0.837] Spawn Actor, and bind event
  (bind _objectinstance (CallFunction|FindPersistentModObjectbyClass "/Game/Mods/braidy08mods/HeistJukeboxRecode/HeistSoundtrackPersistentObject.HeistSoundtrackPersistentObject_C"))
  (bind _asheist_soundtrack_persistent_object (Utilities|Casting|CastToHeistSoundtrackPersistentObject _objectinstance)
    (:then
      (Variables|Default|SetAs%20Heist%20Soundtrack%20Persistent%20Object _asheist_soundtrack_persistent_object)
      (Variables|Default|SetIndex (Variables|/Game/Mods/braidy08mods/HeistJukeboxRecode/HeistSoundtrackPersistentObject.HeistSoundtrackPersistentObject_C|GetIndex (Variables|Default|GetAs%20Heist%20Soundtrack%20Persistent%20Object)))
      (CallFunction|LoadAllPossibleSoundtracks)
      (CallFunction|SetInitialPDAHeist)
      (EventDispatchers|AssignOnStateMachineEnteredLobby (Class|SBZGameStateMachineFunctionLibrary|GetGameStateMachine) (delegate Custom|OnStateMachineEnteredLobby_Event_0))
      ;[1 1 1] saving system
      (bind _returnvalue (SaveGame|DoesSaveGameExist "HeistJukeboxSaveGame"))
      (if _returnvalue
        (bind _returnvalue_2 (SaveGame|LoadGamefromSlot "HeistJukeboxSaveGame"))
        (bind _asheist_jukebox_save_game (Utilities|Casting|CastToHeistJukeboxSaveGame _returnvalue_2))
        (Variables|Default|SetSave _asheist_jukebox_save_game)
        (CallFunction|LoadSave)
        (Utilities|FlowControl|Delay 0.2)
        (if (not (Variables|Default|Getloaded))
          (SaveGame|DeleteGameinSlot "HeistJukeboxSaveGame")
          (Variables|Default|Setloaded true)
          (bind _returnvalue_3 (SaveGame|CreateSaveGameObject "/Game/Mods/braidy08mods/HeistJukeboxRecode/HeistJukeboxSaveGame.HeistJukeboxSaveGame_C" :!label _label))
          (bind _output_get (Variables|Default|SetSave _returnvalue_3))
          (Variables|/Game/Mods/braidy08mods/HeistJukeboxRecode/HeistJukeboxSaveGame.HeistJukeboxSaveGame_C|SetExists _output_get true)
          (SaveGame|SaveGametoSlot _output_get "HeistJukeboxSaveGame"))
        (else
          (goto _label))))
    (:CastFailed
      (CallFunction|PrinttoModLoader "FAILED TO FIND HEIST SOUNDTRACK OBJECT"))))

(fn ConstructionScript
  (|CallParentFunction))

(fn CreateHeistSoundtrackArray
  (return (Utilities|Array|MakeArray (Utilities|Struct|MakeHeistSoundtrackStructure 0 0 "/Game/WWiseAudio/Events/Music/Heists/MusicHeist_03_BranchBank.MusicHeist_03_BranchBank" "No Rest For The Wicked") (Utilities|Struct|MakeHeistSoundtrackStructure 0 0 "/Game/WWiseAudio/Events/Music/Heists/MusicHeist_04_ArmoredTransport.MusicHeist_04_ArmoredTransport" "Road Rage") (Utilities|Struct|MakeHeistSoundtrackStructure 0 0 "/Game/WWiseAudio/Events/Music/Heists/MusicHeist_02_JewelryStore.MusicHeist_02_JewelryStore" "Dirty Ice") (Utilities|Struct|MakeHeistSoundtrackStructure 0 0 "/Game/WWiseAudio/Events/Music/Heists/MusicHeist_08_Nightclub.MusicHeist_08_Nightclub" "Rock The Cradle") (Utilities|Struct|MakeHeistSoundtrackStructure 0 0 "/Game/WWiseAudio/Events/Music/Heists/MusicHeist_07_ArtGallery.MusicHeist_07_ArtGallery" "Under The Surphaze") (Utilities|Struct|MakeHeistSoundtrackStructure 0 0 "/Game/WWiseAudio/Events/Music/Heists/MusicHeist_01_FirstPlayable.MusicHeist_01_FirstPlayable" "Gold & Sharke") (Utilities|Struct|MakeHeistSoundtrackStructure 0 0 "/Game/WWiseAudio/Events/Music/Heists/MusicHeist_05_CargoDocks.MusicHeist_05_CargoDocks" "99 Boxes") (Utilities|Struct|MakeHeistSoundtrackStructure 0 0 "/Game/WWiseAudio/Events/Music/Heists/MusicHeist_06_Penthouse.MusicHeist_06_Penthouse" "Touch The Sky"))))

(fn GetCurrentSoundtrackChoice
  (params (Index :type Integer))
  (return (Utilities|Array|Get(acopy) (Variables|Default|GetHeistSoundtrackArray) Index)))

(fn LoadAllPossibleSoundtracks
  (bind _returnvalue (Class|AssetRegistryHelpers|GetAssetRegistry))
  (bind _as_heist_soundtrack_persistent_object (Variables|Default|GetAs%20Heist%20Soundtrack%20Persistent%20Object))
  (bind _pdaheistsoundtrackarray (Variables|/Game/Mods/braidy08mods/HeistJukeboxRecode/HeistSoundtrackPersistentObject.HeistSoundtrackPersistentObject_C|GetPDAHeistSoundtrackarray _as_heist_soundtrack_persistent_object))
  (Class|AssetRegistry|ScanPathsSynchronous _returnvalue (Utilities|Array|MakeArray "/Game/Mods/HeistJukebox/Music") false)
  (bind _outassetdata (Class|AssetRegistry|GetAssets _returnvalue (Utilities|MakeARFilter 0 (Utilities|Array|MakeArray "/Game/Mods/HeistJukebox/Music") 0 (Utilities|Array|MakeArray "BlueprintGeneratedClass") 0 true true)))
  (for _array_element _outassetdata
    (bind _returnvalue_2 (Utilities|LoadAssetBlocking (Class|KismetSystemLibrary|ToSoftObjRef(SoftObjPath) (Utilities|MakeSoftObjectPath (Utilities|String|Replace (Class|KismetSystemLibrary|GetPathName (Class|AssetRegistryHelpers|GetAsset _array_element)) "." ".Default__")))))
    (bind _aspda_heist_soundtrack (Utilities|Casting|CastToPDA_HeistSoundtrack _returnvalue_2)
      (:then
        (Utilities|Array|AddUnique (Variables|Default|GetPDAHeistSoundtrackarray) _aspda_heist_soundtrack))
      (:CastFailed
        (CallFunction|PrinttoModLoader "FAILED TO CAST ASSET!!"))))
  (Utilities|Array|Clear _pdaheistsoundtrackarray)
  (Utilities|Array|AppendArray _pdaheistsoundtrackarray (Variables|Default|GetPDAHeistSoundtrackarray)))

(fn GetCurrentPDA
  (params (Index :type Integer))
  (return (Utilities|Array|Get(acopy) (Variables|Default|GetPDAHeistSoundtrackarray) Index)))

(fn SetInitialPDAHeist
  (Variables|/Game/Mods/braidy08mods/HeistJukeboxRecode/HeistSoundtrackPersistentObject.HeistSoundtrackPersistentObject_C|SetPDAHeist (Variables|Default|GetAs%20Heist%20Soundtrack%20Persistent%20Object) (Utilities|Array|Get(acopy) (Variables|Default|GetPDAHeistSoundtrackarray) (Variables|Default|GetIndex))))

(fn LoadSave
  (bind _save (Variables|Default|GetSave))
  (bind _as_heist_soundtrack_persistent_object (Variables|Default|GetAs%20Heist%20Soundtrack%20Persistent%20Object))
  (Variables|Default|Setloaded (Variables|/Game/Mods/braidy08mods/HeistJukeboxRecode/HeistJukeboxSaveGame.HeistJukeboxSaveGame_C|GetExists _save))
  (bind _output_get (Variables|/Game/Mods/braidy08mods/HeistJukeboxRecode/HeistSoundtrackPersistentObject.HeistSoundtrackPersistentObject_C|SetassaultRandomSong _as_heist_soundtrack_persistent_object (Variables|/Game/Mods/braidy08mods/HeistJukeboxRecode/HeistJukeboxSaveGame.HeistJukeboxSaveGame_C|GetRandomAssaultEnabled _save)))
  (bind _output_get_2 (Variables|/Game/Mods/braidy08mods/HeistJukeboxRecode/HeistSoundtrackPersistentObject.HeistSoundtrackPersistentObject_C|SetrandomSong _as_heist_soundtrack_persistent_object (Variables|/Game/Mods/braidy08mods/HeistJukeboxRecode/HeistJukeboxSaveGame.HeistJukeboxSaveGame_C|GetRandomEnabled _save)))
  (bind _output_get_3 (Variables|/Game/Mods/braidy08mods/HeistJukeboxRecode/HeistSoundtrackPersistentObject.HeistSoundtrackPersistentObject_C|SetEnableRTCStealth _as_heist_soundtrack_persistent_object (Variables|/Game/Mods/braidy08mods/HeistJukeboxRecode/HeistJukeboxSaveGame.HeistJukeboxSaveGame_C|GetRTCStealthEnabled _save)))
  (bind _output_get_4 (Variables|/Game/Mods/braidy08mods/HeistJukeboxRecode/HeistSoundtrackPersistentObject.HeistSoundtrackPersistentObject_C|SetdisableRTCFix _as_heist_soundtrack_persistent_object (Variables|/Game/Mods/braidy08mods/HeistJukeboxRecode/HeistJukeboxSaveGame.HeistJukeboxSaveGame_C|GetRTCFixDisabled _save)))
  (Default|LoadSaveUI (Variables|Default|GetSoundtrack%20Selector%20Widget) _output_get _output_get_2 _output_get_3 _output_get_4))

(fn SaveSave
  (bind _save (Variables|Default|GetSave))
  (bind _as_heist_soundtrack_persistent_object (Variables|Default|GetAs%20Heist%20Soundtrack%20Persistent%20Object))
  (Variables|/Game/Mods/braidy08mods/HeistJukeboxRecode/HeistJukeboxSaveGame.HeistJukeboxSaveGame_C|SetRandomAssaultEnabled _save (Variables|/Game/Mods/braidy08mods/HeistJukeboxRecode/HeistSoundtrackPersistentObject.HeistSoundtrackPersistentObject_C|GetassaultRandomSong _as_heist_soundtrack_persistent_object))
  (Variables|/Game/Mods/braidy08mods/HeistJukeboxRecode/HeistJukeboxSaveGame.HeistJukeboxSaveGame_C|SetRandomEnabled _save (Variables|/Game/Mods/braidy08mods/HeistJukeboxRecode/HeistSoundtrackPersistentObject.HeistSoundtrackPersistentObject_C|GetrandomSong _as_heist_soundtrack_persistent_object))
  (Variables|/Game/Mods/braidy08mods/HeistJukeboxRecode/HeistJukeboxSaveGame.HeistJukeboxSaveGame_C|SetRTCStealthEnabled _save (Variables|/Game/Mods/braidy08mods/HeistJukeboxRecode/HeistSoundtrackPersistentObject.HeistSoundtrackPersistentObject_C|GetEnableRTCStealth _as_heist_soundtrack_persistent_object))
  (Variables|/Game/Mods/braidy08mods/HeistJukeboxRecode/HeistJukeboxSaveGame.HeistJukeboxSaveGame_C|SetRTCFixDisabled _save (Variables|/Game/Mods/braidy08mods/HeistJukeboxRecode/HeistSoundtrackPersistentObject.HeistSoundtrackPersistentObject_C|GetdisableRTCFix _as_heist_soundtrack_persistent_object))
  (SaveGame|SaveGametoSlot _save "HeistJukeboxSaveGame"))

(fn SetDefaultPDAPerHeist
  (bind _dt_basegamesoundtracks (Variables|Default|GetDT_BasegameSoundtracks))
  (bind _as_heist_soundtrack_persistent_object (Variables|Default|GetAs%20Heist%20Soundtrack%20Persistent%20Object))
  (bind _outrownames (DataTable|GetDataTableRowNames _dt_basegamesoundtracks))
  (for _array_element _outrownames
    (bind _returnvalue (Utilities|GetDataTableRow _dt_basegamesoundtracks _array_element)
      (:then
        (if (== (.HeistIDX (Utilities|Struct|BreakHeistSoundtrackStructure _returnvalue)) (Class|SBZGameStateMachine|GetMatchmakingLevelIdx (Class|SBZGameStateMachineFunctionLibrary|GetGameStateMachine)))
          (for (_array_element_2 _array_index) (Variables|Default|GetPDAHeistSoundtrackarray)
            (if (Utilities|ClassIsChildOf (Utilities|GetClass _array_element_2) (.SoundtrackPDA (Utilities|Struct|BreakHeistSoundtrackStructure _returnvalue)))
              (bind _output_get (Variables|Default|SetIndex _array_index))
              (Variables|/Game/Mods/braidy08mods/HeistJukeboxRecode/HeistSoundtrackPersistentObject.HeistSoundtrackPersistentObject_C|SetIndex _as_heist_soundtrack_persistent_object _output_get)
              (Variables|/Game/Mods/braidy08mods/HeistJukeboxRecode/HeistSoundtrackPersistentObject.HeistSoundtrackPersistentObject_C|SetPDAHeist _as_heist_soundtrack_persistent_object _array_element_2)
              (return))))))))

(fn SetupPreLobby)