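; Payday 3 Heist Jukebox mod actor that replaces a heist's music with the player's chosen, random or playlist track, skipping tutorial levels.
; BeginPlay reads settings and songs from the persistent mod object, with a special music fix for RTC.
; Heist-state and gone-loud events swap out stealth-only tracks, optionally reroll after assaults, and cycle songs on a random timer from Point of No Return.
; A widget displays the current song.
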(event Custom|EventOnHeistGoneLoud_0
  (bind _returnvalue (Class|SBZMusicManager|GetMusicManager))
  (bind _returnvalue_2 (Class|SBZMusicManager|GetMusicManager))
  (bind _as_heist_soundtrack_persistent_object (Variables|Default|GetAs%20Heist%20Soundtrack%20Persistent%20Object))
  (bind _as_heist_soundtrack_persistent_object_2 (Variables|Default|GetAs%20Heist%20Soundtrack%20Persistent%20Object))
  ;[1 1 1] dont even know the point of this
  (Class|SBZMusicManager|StopMusic _returnvalue)
  (Class|SBZMusicManager|PlayMusic _returnvalue (Variables|/Game/Mods/HeistJukebox/PDA_HeistSoundtrack.PDA_HeistSoundtrack_C|GetAudio%20Event (Variables|/Game/Mods/braidy08mods/HeistJukeboxRecode/HeistSoundtrackPersistentObject.HeistSoundtrackPersistentObject_C|GetPDAHeist _as_heist_soundtrack_persistent_object_2)) false)
  (if (Variables|/Game/Mods/HeistJukebox/PDA_HeistSoundtrack.PDA_HeistSoundtrack_C|GetStealth%20Only (Variables|/Game/Mods/braidy08mods/HeistJukeboxRecode/HeistSoundtrackPersistentObject.HeistSoundtrackPersistentObject_C|GetPDAHeist _as_heist_soundtrack_persistent_object_2))
    ;[1 1 1] playsongshit
    (bind _returnvalue_3 (Actor|GetActorOfClass "/Script/Starbreeze.PD3HeistGameState"))
    (if (Utilities|Enum|Equal(Enum) (Class|PD3HeistGameState|GetCurrentHeistState _returnvalue_3) "Stealth")
      (bind _outactors (Actor|GetAllActorsOfClass "/Script/Starbreeze.PD3HeistGameState" :!label _label))
      (EventDispatchers|AssignOnHeistStateChanged _outactors (EventDispatchers|CreateEvent :!event Custom|OnHeistStateChanged_Event_0))
      (elif (Utilities|Enum|Equal(Enum) (Class|PD3HeistGameState|GetCurrentHeistState _returnvalue_3) "Search")
        (goto _label)
        (elif (not (Variables|/Game/Mods/braidy08mods/HeistJukeboxRecode/HeistSoundtrackPersistentObject.HeistSoundtrackPersistentObject_C|GetplaylistEnabled (Variables|Default|GetAs%20Heist%20Soundtrack%20Persistent%20Object)))
          ;[1 1 1] random assault shit
          (Variables|/Game/Mods/braidy08mods/HeistJukeboxRecode/HeistSoundtrackPersistentObject.HeistSoundtrackPersistentObject_C|SetPDAHeist _as_heist_soundtrack_persistent_object (.OutItem (Utilities|Array|Random (Variables|Default|GetPDAHeistSoundtrackarray))) :!label _label_2)
          (if (Variables|/Game/Mods/HeistJukebox/PDA_HeistSoundtrack.PDA_HeistSoundtrack_C|GetStealth%20Only (Variables|/Game/Mods/braidy08mods/HeistJukeboxRecode/HeistSoundtrackPersistentObject.HeistSoundtrackPersistentObject_C|GetPDAHeist _as_heist_soundtrack_persistent_object))
            (goto _label_2)
            (else
              (Class|SBZMusicManager|StopMusic _returnvalue_2)
              (Class|SBZMusicManager|PlayMusic _returnvalue_2 (Variables|/Game/Mods/HeistJukebox/PDA_HeistSoundtrack.PDA_HeistSoundtrack_C|GetAudio%20Event (Variables|/Game/Mods/braidy08mods/HeistJukeboxRecode/HeistSoundtrackPersistentObject.HeistSoundtrackPersistentObject_C|GetPDAHeist _as_heist_soundtrack_persistent_object)) false))))))
    (elif (Variables|/Game/Mods/braidy08mods/HeistJukeboxRecode/HeistSoundtrackPersistentObject.HeistSoundtrackPersistentObject_C|GetassaultRandomSong _as_heist_soundtrack_persistent_object_2)
      (goto _label))))

(event Custom|OnHeistStateChanged_Event_0
  (params (OldState :type EPD3HeistState%20Enum :default "Stealth") (NewState :type EPD3HeistState%20Enum :default "Stealth"))
  (bind _returnvalue (Class|SBZMusicManager|GetMusicManager))
  (bind _returnvalue_2 (Class|SBZMusicManager|GetMusicManager))
  (bind _returnvalue_3 (Class|SBZMusicManager|GetMusicManager))
  (bind _returnvalue_4 (Class|SBZGameStateMachineFunctionLibrary|GetGameStateMachineState))
  (bind _returnvalue_5 (Class|SBZMusicManager|GetMusicManager))
  (bind _returnvalue_6 (Class|SBZMusicManager|GetMusicManager))
  (bind _returnvalue_7 (Math|Random|RandomFloatinRange 1.2e+02 2.4e+02))
  (bind _as_heist_soundtrack_persistent_object (Variables|Default|GetAs%20Heist%20Soundtrack%20Persistent%20Object))
  (bind _as_heist_soundtrack_persistent_object_2 (Variables|Default|GetAs%20Heist%20Soundtrack%20Persistent%20Object))
  (bind _as_heist_soundtrack_persistent_object_3 (Variables|Default|GetAs%20Heist%20Soundtrack%20Persistent%20Object))
  (bind _as_heist_soundtrack_persistent_object_4 (Variables|Default|GetAs%20Heist%20Soundtrack%20Persistent%20Object))
  (bind _as_heist_soundtrack_persistent_object_5 (Variables|Default|GetAs%20Heist%20Soundtrack%20Persistent%20Object))
  (bind _as_heist_soundtrack_persistent_object_6 (Variables|Default|GetAs%20Heist%20Soundtrack%20Persistent%20Object))
  (bind _as_heist_soundtrack_persistent_object_7 (Variables|Default|GetAs%20Heist%20Soundtrack%20Persistent%20Object))
  (bind _returnvalue_8 (Utilities|Enum|Equal(Enum) _returnvalue_4 "SM_Result"))
  (bind _playlistenabled (Variables|/Game/Mods/braidy08mods/HeistJukeboxRecode/HeistSoundtrackPersistentObject.HeistSoundtrackPersistentObject_C|GetplaylistEnabled _as_heist_soundtrack_persistent_object_7))
  (bind _assaultrandomsong (Variables|/Game/Mods/braidy08mods/HeistJukeboxRecode/HeistSoundtrackPersistentObject.HeistSoundtrackPersistentObject_C|GetassaultRandomSong _as_heist_soundtrack_persistent_object_5))
  (Utilities|FlowControl|Sequence
    (:then_0
      (bind _output_get (Variables|Default|Setcurrentstatereal NewState))
      (if (Variables|/Game/Mods/braidy08mods/HeistJukeboxRecode/HeistSoundtrackPersistentObject.HeistSoundtrackPersistentObject_C|GetHeistIsRTC _as_heist_soundtrack_persistent_object_7)
        (if (Utilities|Enum|Equal(Enum) NewState "Alarm")
          ;[1 1 1] rtc fix
          (Utilities|FlowControl|Delay 0.2)
          (Class|SBZMusicManager|StopMusic _returnvalue_3)
          (Class|SBZMusicManager|PlayMusic _returnvalue_3 "/Game/WWiseAudio/Events/Music/System/Music_Stop_Nightclub_Diagetic.Music_Stop_Nightclub_Diagetic" false)
          (if (Variables|/Game/Mods/HeistJukebox/PDA_HeistSoundtrack.PDA_HeistSoundtrack_C|GetStealth%20Only (Variables|/Game/Mods/braidy08mods/HeistJukeboxRecode/HeistSoundtrackPersistentObject.HeistSoundtrackPersistentObject_C|GetPDAHeist _as_heist_soundtrack_persistent_object_6))
            (Variables|/Game/Mods/braidy08mods/HeistJukeboxRecode/HeistSoundtrackPersistentObject.HeistSoundtrackPersistentObject_C|SetPDAHeist _as_heist_soundtrack_persistent_object (.OutItem (Utilities|Array|Random (Variables|Default|GetPDAHeistSoundtrackarray))) :!label _label)
            (if (Variables|/Game/Mods/HeistJukebox/PDA_HeistSoundtrack.PDA_HeistSoundtrack_C|GetStealth%20Only (Variables|/Game/Mods/braidy08mods/HeistJukeboxRecode/HeistSoundtrackPersistentObject.HeistSoundtrackPersistentObject_C|GetPDAHeist _as_heist_soundtrack_persistent_object))
              (goto _label)
              (else
                _)))
          (Class|SBZMusicManager|StopMusic _returnvalue_5)
          (Class|SBZMusicManager|PlayMusic _returnvalue_5 (Variables|/Game/Mods/HeistJukebox/PDA_HeistSoundtrack.PDA_HeistSoundtrack_C|GetAudio%20Event (Variables|/Game/Mods/braidy08mods/HeistJukeboxRecode/HeistSoundtrackPersistentObject.HeistSoundtrackPersistentObject_C|GetPDAHeist _as_heist_soundtrack_persistent_object_6)) false)
          (Variables|/Game/Mods/braidy08mods/HeistJukeboxRecode/HeistSoundtrackPersistentObject.HeistSoundtrackPersistentObject_C|SetHeistIsRTC _as_heist_soundtrack_persistent_object_6 false))
        (else
          (switch Utilities|FlowControl|Switch|SwitchonEPD3HeistState _output_get
            (:Alarm
              ;[1 1 1] playlist shit
              (if _playlistenabled
                (if (Variables|/Game/Mods/HeistJukebox/PDA_HeistSoundtrack.PDA_HeistSoundtrack_C|GetStealth%20Only (Variables|/Game/Mods/braidy08mods/HeistJukeboxRecode/HeistSoundtrackPersistentObject.HeistSoundtrackPersistentObject_C|GetPDAHeist (Variables|Default|GetAs%20Heist%20Soundtrack%20Persistent%20Object))) :!label _label_2
                  (Variables|/Game/Mods/braidy08mods/HeistJukeboxRecode/HeistSoundtrackPersistentObject.HeistSoundtrackPersistentObject_C|SetPDAHeist _as_heist_soundtrack_persistent_object_2 (.OutItem (Utilities|Array|Random (Variables|/Game/Mods/braidy08mods/HeistJukeboxRecode/HeistSoundtrackPersistentObject.HeistSoundtrackPersistentObject_C|GetPDAHeistPlaylistArray _as_heist_soundtrack_persistent_object_2))) :!label _label_3)
                  (if (Variables|/Game/Mods/HeistJukebox/PDA_HeistSoundtrack.PDA_HeistSoundtrack_C|GetStealth%20Only (Variables|/Game/Mods/braidy08mods/HeistJukeboxRecode/HeistSoundtrackPersistentObject.HeistSoundtrackPersistentObject_C|GetPDAHeist _as_heist_soundtrack_persistent_object_2))
                    (goto _label_3)
                    (else
                      (Class|SBZMusicManager|StopMusic _returnvalue_6)
                      (Class|SBZMusicManager|PlayMusic _returnvalue_6 (Variables|/Game/Mods/HeistJukebox/PDA_HeistSoundtrack.PDA_HeistSoundtrack_C|GetAudio%20Event (Variables|/Game/Mods/braidy08mods/HeistJukeboxRecode/HeistSoundtrackPersistentObject.HeistSoundtrackPersistentObject_C|GetPDAHeist _as_heist_soundtrack_persistent_object_2)) false))))
                (else
                  ;[1 1 1] random assault shit
                  (if (Variables|/Game/Mods/HeistJukebox/PDA_HeistSoundtrack.PDA_HeistSoundtrack_C|GetStealth%20Only (Variables|/Game/Mods/braidy08mods/HeistJukeboxRecode/HeistSoundtrackPersistentObject.HeistSoundtrackPersistentObject_C|GetPDAHeist (Variables|Default|GetAs%20Heist%20Soundtrack%20Persistent%20Object))) :!label _label_4
                    (Variables|/Game/Mods/braidy08mods/HeistJukeboxRecode/HeistSoundtrackPersistentObject.HeistSoundtrackPersistentObject_C|SetPDAHeist _as_heist_soundtrack_persistent_object_4 (.OutItem (Utilities|Array|Random (Variables|Default|GetPDAHeistSoundtrackarray))) :!label _label_5)
                    (if (Variables|/Game/Mods/HeistJukebox/PDA_HeistSoundtrack.PDA_HeistSoundtrack_C|GetStealth%20Only (Variables|/Game/Mods/braidy08mods/HeistJukeboxRecode/HeistSoundtrackPersistentObject.HeistSoundtrackPersistentObject_C|GetPDAHeist _as_heist_soundtrack_persistent_object_4))
                      (goto _label_5)
                      (else
                        (Class|SBZMusicManager|StopMusic _returnvalue_2)
                        (Class|SBZMusicManager|PlayMusic _returnvalue_2 (Variables|/Game/Mods/HeistJukebox/PDA_HeistSoundtrack.PDA_HeistSoundtrack_C|GetAudio%20Event (Variables|/Game/Mods/braidy08mods/HeistJukeboxRecode/HeistSoundtrackPersistentObject.HeistSoundtrackPersistentObject_C|GetPDAHeist _as_heist_soundtrack_persistent_object_4)) false)))))))
            (:Anticipation
              (if _playlistenabled
                (goto _label_2)
                (else
                  (goto _label_4))))
            (:Assault
              (if _playlistenabled
                (if (Variables|/Game/Mods/HeistJukebox/PDA_HeistSoundtrack.PDA_HeistSoundtrack_C|GetStealth%20Only (Variables|/Game/Mods/braidy08mods/HeistJukeboxRecode/HeistSoundtrackPersistentObject.HeistSoundtrackPersistentObject_C|GetPDAHeist (Variables|Default|GetAs%20Heist%20Soundtrack%20Persistent%20Object)))
                  (goto _label_3)
                  (elif (not (Variables|Default|Getassaultyes))
                    (Variables|Default|Setassaultyes true)))
                (elif (Variables|/Game/Mods/HeistJukebox/PDA_HeistSoundtrack.PDA_HeistSoundtrack_C|GetStealth%20Only (Variables|/Game/Mods/braidy08mods/HeistJukeboxRecode/HeistSoundtrackPersistentObject.HeistSoundtrackPersistentObject_C|GetPDAHeist (Variables|Default|GetAs%20Heist%20Soundtrack%20Persistent%20Object)))
                  (goto _label_5)
                  (elif _assaultrandomsong
                    (if (not (Variables|Default|Getassaultyes))
                      (Variables|Default|Setassaultyes true))))))
            (:Control
              (if _playlistenabled
                (if (Variables|/Game/Mods/HeistJukebox/PDA_HeistSoundtrack.PDA_HeistSoundtrack_C|GetStealth%20Only (Variables|/Game/Mods/braidy08mods/HeistJukeboxRecode/HeistSoundtrackPersistentObject.HeistSoundtrackPersistentObject_C|GetPDAHeist (Variables|Default|GetAs%20Heist%20Soundtrack%20Persistent%20Object)))
                  (goto _label_3)
                  (elif (Variables|Default|Getassaultyes)
                    (Variables|Default|Setassaultyes false)
                    (goto _label_3)))
                (elif (Variables|/Game/Mods/HeistJukebox/PDA_HeistSoundtrack.PDA_HeistSoundtrack_C|GetStealth%20Only (Variables|/Game/Mods/braidy08mods/HeistJukeboxRecode/HeistSoundtrackPersistentObject.HeistSoundtrackPersistentObject_C|GetPDAHeist (Variables|Default|GetAs%20Heist%20Soundtrack%20Persistent%20Object)))
                  (goto _label_5)
                  (elif _assaultrandomsong
                    (if (Variables|Default|Getassaultyes)
                      (Variables|Default|Setassaultyes false)
                      (goto _label_5))))))
            (:PointOfNoReturn
              ;[1 1 1] finalassault crap
              (if _playlistenabled
                (Variables|/Game/Mods/braidy08mods/HeistJukeboxRecode/HeistSoundtrackPersistentObject.HeistSoundtrackPersistentObject_C|SetPDAHeist _as_heist_soundtrack_persistent_object_3 (.OutItem (Utilities|Array|Random (Variables|/Game/Mods/braidy08mods/HeistJukeboxRecode/HeistSoundtrackPersistentObject.HeistSoundtrackPersistentObject_C|GetPDAHeistPlaylistArray _as_heist_soundtrack_persistent_object_3))) :!label _label_6)
                (if (Variables|/Game/Mods/HeistJukebox/PDA_HeistSoundtrack.PDA_HeistSoundtrack_C|GetStealth%20Only (Variables|/Game/Mods/braidy08mods/HeistJukeboxRecode/HeistSoundtrackPersistentObject.HeistSoundtrackPersistentObject_C|GetPDAHeist _as_heist_soundtrack_persistent_object_3))
                  (goto _label_6)
                  (else
                    (Class|SBZMusicManager|StopMusic _returnvalue :!label _label_7)
                    (Class|SBZMusicManager|PlayMusic _returnvalue (Variables|/Game/Mods/HeistJukebox/PDA_HeistSoundtrack.PDA_HeistSoundtrack_C|GetAudio%20Event (Variables|/Game/Mods/braidy08mods/HeistJukeboxRecode/HeistSoundtrackPersistentObject.HeistSoundtrackPersistentObject_C|GetPDAHeist _as_heist_soundtrack_persistent_object_3)) false)
                    (Utilities|FlowControl|Sequence
                      (:then_0
                        ;[1 1 1] currentsonghud
                        (Class|UserWidget|PlayAnimationForward (stale EventBeginPlay _output_get_2) (Variables|/Game/Mods/LegacyHeistJukebox/WBP_CurrentSong.WBP_CurrentSong_C|GetTextChange (stale EventBeginPlay _output_get_2)) 1.0 true :!label _label_8)
                        (Utilities|FlowControl|Delay 0.15)
                        (Default|SetCurrentPlayingText (stale EventBeginPlay _output_get_2) (Variables|/Game/Mods/HeistJukebox/PDA_HeistSoundtrack.PDA_HeistSoundtrack_C|GetName (Variables|/Game/Mods/braidy08mods/HeistJukeboxRecode/HeistSoundtrackPersistentObject.HeistSoundtrackPersistentObject_C|GetPDAHeist (Variables|Default|GetAs%20Heist%20Soundtrack%20Persistent%20Object)))))
                      (:then_1
                        (if (Variables|/Game/Mods/braidy08mods/HeistJukeboxRecode/HeistSoundtrackPersistentObject.HeistSoundtrackPersistentObject_C|GetplaylistEnabled _as_heist_soundtrack_persistent_object_3)
                          (Utilities|FlowControl|Delay _returnvalue_7)
                          (if (not _returnvalue_8)
                            (goto _label_6))
                          (else
                            (Utilities|FlowControl|Delay _returnvalue_7)
                            (if (not _returnvalue_8)
                              (Variables|/Game/Mods/braidy08mods/HeistJukeboxRecode/HeistSoundtrackPersistentObject.HeistSoundtrackPersistentObject_C|SetPDAHeist _as_heist_soundtrack_persistent_object_3 (.OutItem (Utilities|Array|Random (Variables|Default|GetPDAHeistSoundtrackarray))) :!label _label_9)
                              (if (Variables|/Game/Mods/HeistJukebox/PDA_HeistSoundtrack.PDA_HeistSoundtrack_C|GetStealth%20Only (Variables|/Game/Mods/braidy08mods/HeistJukeboxRecode/HeistSoundtrackPersistentObject.HeistSoundtrackPersistentObject_C|GetPDAHeist _as_heist_soundtrack_persistent_object_3))
                                (goto _label_9)
                                (else
                                  (goto _label_7))))))))))
                (else
                  (goto _label_9))))))))
    (:then_1
      (goto _label_8))))

(event EventBeginPlay
  (bind _returnvalue (Class|SBZMusicManager|GetMusicManager))
  (bind _returnvalue_2 (Class|SBZMusicManager|GetMusicManager))
  (bind _returnvalue_3 (Class|SBZMusicManager|GetMusicManager))
  (bind _returnvalue_4 (Class|SBZMusicManager|GetMusicManager))
  (bind _returnvalue_5 (Class|SBZMusicManager|GetMusicManager))
  (bind _returnvalue_6 (Class|SBZMusicManager|GetMusicManager))
  (bind _objectinstance (CallFunction|FindPersistentModObjectbyClass "/Game/Mods/braidy08mods/HeistJukeboxRecode/HeistSoundtrackPersistentObject.HeistSoundtrackPersistentObject_C"))
  (bind _asheist_soundtrack_persistent_object (Utilities|Casting|CastToHeistSoundtrackPersistentObject _objectinstance)
    (:then
      (Variables|Default|SetAs%20Heist%20Soundtrack%20Persistent%20Object _asheist_soundtrack_persistent_object)
      (CallFunction|LoadSongs)
      (bind _heistpda (CallFunction|GetSongatIndex (Variables|/Game/Mods/braidy08mods/HeistJukeboxRecode/HeistSoundtrackPersistentObject.HeistSoundtrackPersistentObject_C|GetIndex (Variables|Default|GetAs%20Heist%20Soundtrack%20Persistent%20Object))))
      (Variables|/Game/Mods/braidy08mods/HeistJukeboxRecode/HeistSoundtrackPersistentObject.HeistSoundtrackPersistentObject_C|SetPDAHeist (Variables|Default|GetAs%20Heist%20Soundtrack%20Persistent%20Object) _heistpda)
      (if (Variables|/Game/Mods/braidy08mods/HeistJukeboxRecode/HeistSoundtrackPersistentObject.HeistSoundtrackPersistentObject_C|Getdebug (Variables|Default|GetAs%20Heist%20Soundtrack%20Persistent%20Object))
        (CallFunction|PrinttoModLoader (Utilities|String|Append (Utilities|String|Append "Debug: " (Utilities|String|ToString(Boolean) (Variables|/Game/Mods/braidy08mods/HeistJukeboxRecode/HeistSoundtrackPersistentObject.HeistSoundtrackPersistentObject_C|Getdebug (Variables|Default|GetAs%20Heist%20Soundtrack%20Persistent%20Object)))) "," (Utilities|String|ToString(Text) (Variables|/Game/Mods/HeistJukebox/PDA_HeistSoundtrack.PDA_HeistSoundtrack_C|GetName (Variables|/Game/Mods/braidy08mods/HeistJukeboxRecode/HeistSoundtrackPersistentObject.HeistSoundtrackPersistentObject_C|GetPDAHeist (Variables|Default|GetAs%20Heist%20Soundtrack%20Persistent%20Object)))) "," (Utilities|GetDisplayName (Variables|/Game/Mods/HeistJukebox/PDA_HeistSoundtrack.PDA_HeistSoundtrack_C|GetAudio%20Event (Variables|/Game/Mods/braidy08mods/HeistJukeboxRecode/HeistSoundtrackPersistentObject.HeistSoundtrackPersistentObject_C|GetPDAHeist (Variables|Default|GetAs%20Heist%20Soundtrack%20Persistent%20Object)))) "," (Utilities|String|Append "Playlist Enabled: " (Utilities|String|ToString(Boolean) (Variables|/Game/Mods/braidy08mods/HeistJukeboxRecode/HeistSoundtrackPersistentObject.HeistSoundtrackPersistentObject_C|GetplaylistEnabled (Variables|Default|GetAs%20Heist%20Soundtrack%20Persistent%20Object)))))))
      (if (not (Variables|/Game/Mods/braidy08mods/HeistJukeboxRecode/HeistSoundtrackPersistentObject.HeistSoundtrackPersistentObject_C|GetJukeboxDisabled (Variables|Default|GetAs%20Heist%20Soundtrack%20Persistent%20Object)))
        (bind _returnvalue_7 (Game|GetCurrentLevelName true))
        (if (not (Variables|/Script/Starbreeze.PD3HeistDataAsset|GetbIsTutorialLevel (Class|SBZHeistDeveloperSettings|GetHeistDatafromLevelShortName _returnvalue_7)))
          (Utilities|FlowControl|Sequence
            (:then_0
              (bind _returnvalue_8 (Game|GetCurrentLevelName true))
              (if (== (Class|SBZGameStateMachineSettings|LevelShortNametoIdx _returnvalue_8) 3)
                (Variables|/Game/Mods/braidy08mods/HeistJukeboxRecode/HeistSoundtrackPersistentObject.HeistSoundtrackPersistentObject_C|SetHeistIsRTC (Variables|Default|GetAs%20Heist%20Soundtrack%20Persistent%20Object) true))
              (if (Variables|/Game/Mods/braidy08mods/HeistJukeboxRecode/HeistSoundtrackPersistentObject.HeistSoundtrackPersistentObject_C|GetplaylistEnabled (Variables|Default|GetAs%20Heist%20Soundtrack%20Persistent%20Object))
                ;[1 1 1] playlist
                (if (Class|SBZOnlineFunctionLibrary|IsSoloGame)
                  (if (Utilities|Enum|Equal(Enum) (Class|SBZGameStateMachineFunctionLibrary|GetGameStateMachineState) "SM_ActionPhase") :!label _label
                    _
                    (else
                      (Utilities|FlowControl|Delay 0.2)
                      (goto _label))))
                (Utilities|FlowControl|Delay 0.2)
                (bind _output_get (Variables|/Game/Mods/braidy08mods/HeistJukeboxRecode/HeistSoundtrackPersistentObject.HeistSoundtrackPersistentObject_C|SetPDAHeist (Variables|Default|GetAs%20Heist%20Soundtrack%20Persistent%20Object) (.OutItem (Utilities|Array|Random (Variables|/Game/Mods/braidy08mods/HeistJukeboxRecode/HeistSoundtrackPersistentObject.HeistSoundtrackPersistentObject_C|GetPDAHeistPlaylistArray (Variables|Default|GetAs%20Heist%20Soundtrack%20Persistent%20Object))))))
                (Class|SBZMusicManager|StopMusic _returnvalue)
                (Class|SBZMusicManager|PlayMusic _returnvalue (Variables|/Game/Mods/HeistJukebox/PDA_HeistSoundtrack.PDA_HeistSoundtrack_C|GetAudio%20Event _output_get) false)
                (Utilities|FlowControl|Sequence
                  (:then_0
                    (bind _outactors (Actor|GetAllActorsOfClass "/Script/Starbreeze.PD3HeistGameState" :!label _label_2))
                    (EventDispatchers|AssignOnHeistStateChanged _outactors (EventDispatchers|CreateEvent :!event Custom|OnHeistStateChanged_Event_0)))
                  (:then_1
                    ;[1 1 1] currentsonghud
                    (Class|UserWidget|PlayAnimationForward (stale _output_get_2) (Variables|/Game/Mods/LegacyHeistJukebox/WBP_CurrentSong.WBP_CurrentSong_C|GetTextChange (stale _output_get_2)) 1.0 true)
                    (Utilities|FlowControl|Delay 0.15)
                    (Default|SetCurrentPlayingText (stale _output_get_2) (Variables|/Game/Mods/HeistJukebox/PDA_HeistSoundtrack.PDA_HeistSoundtrack_C|GetName (Variables|/Game/Mods/braidy08mods/HeistJukeboxRecode/HeistSoundtrackPersistentObject.HeistSoundtrackPersistentObject_C|GetPDAHeist (Variables|Default|GetAs%20Heist%20Soundtrack%20Persistent%20Object))) :!label _label_3)))
                (else
                  (if (Variables|/Game/Mods/braidy08mods/HeistJukeboxRecode/HeistSoundtrackPersistentObject.HeistSoundtrackPersistentObject_C|GetrandomSong (Variables|Default|GetAs%20Heist%20Soundtrack%20Persistent%20Object))
                    (Variables|/Game/Mods/braidy08mods/HeistJukeboxRecode/HeistSoundtrackPersistentObject.HeistSoundtrackPersistentObject_C|SetPDAHeist (Variables|Default|GetAs%20Heist%20Soundtrack%20Persistent%20Object) (.OutItem (Utilities|Array|Random (Variables|Default|GetPDAHeistSoundtrackarray))))
                    (Variables|/Game/Mods/braidy08mods/HeistJukeboxRecode/HeistSoundtrackPersistentObject.HeistSoundtrackPersistentObject_C|SetrandomSong (Variables|Default|GetAs%20Heist%20Soundtrack%20Persistent%20Object) false))
                  (if (Variables|/Game/Mods/braidy08mods/HeistJukeboxRecode/HeistSoundtrackPersistentObject.HeistSoundtrackPersistentObject_C|GetHeistIsRTC (Variables|Default|GetAs%20Heist%20Soundtrack%20Persistent%20Object))
                    (if (Variables|/Game/Mods/braidy08mods/HeistJukeboxRecode/HeistSoundtrackPersistentObject.HeistSoundtrackPersistentObject_C|GetEnableRTCStealth (Variables|Default|GetAs%20Heist%20Soundtrack%20Persistent%20Object))
                      (if (not (Variables|/Game/Mods/braidy08mods/HeistJukeboxRecode/HeistSoundtrackPersistentObject.HeistSoundtrackPersistentObject_C|GetdisableRTCFix (Variables|Default|GetAs%20Heist%20Soundtrack%20Persistent%20Object)))
                        (Variables|/Game/Mods/braidy08mods/HeistJukeboxRecode/HeistSoundtrackPersistentObject.HeistSoundtrackPersistentObject_C|SetHeistIsRTC (Variables|Default|GetAs%20Heist%20Soundtrack%20Persistent%20Object) false)
                        (Class|SBZMusicManager|StopMusic _returnvalue_5)
                        (Class|SBZMusicManager|PlayMusic _returnvalue_5 "/Game/WWiseAudio/Events/Music/System/Music_Stop_Nightclub_Diagetic.Music_Stop_Nightclub_Diagetic" false)
                        (Utilities|FlowControl|Sequence
                          (:then_0
                            (Utilities|FlowControl|Delay 0.2)
                            ;[1 1 1] rtc fix
                            (Class|SBZMusicManager|StopMusic _returnvalue_3 :!label _label_4)
                            (Class|SBZMusicManager|PlayMusic _returnvalue_3 "/Game/WWiseAudio/Events/Music/System/Music_Stop_Nightclub_Diagetic.Music_Stop_Nightclub_Diagetic" false)
                            (if (Variables|/Game/Mods/HeistJukebox/PDA_HeistSoundtrack.PDA_HeistSoundtrack_C|GetStealth%20Only (Variables|/Game/Mods/braidy08mods/HeistJukeboxRecode/HeistSoundtrackPersistentObject.HeistSoundtrackPersistentObject_C|GetPDAHeist (Variables|Default|GetAs%20Heist%20Soundtrack%20Persistent%20Object)))
                              (Variables|/Game/Mods/braidy08mods/HeistJukeboxRecode/HeistSoundtrackPersistentObject.HeistSoundtrackPersistentObject_C|SetPDAHeist (Variables|Default|GetAs%20Heist%20Soundtrack%20Persistent%20Object) (.OutItem (Utilities|Array|Random (Variables|Default|GetPDAHeistSoundtrackarray))) :!label _label_5)
                              (if (Variables|/Game/Mods/HeistJukebox/PDA_HeistSoundtrack.PDA_HeistSoundtrack_C|GetStealth%20Only (Variables|/Game/Mods/braidy08mods/HeistJukeboxRecode/HeistSoundtrackPersistentObject.HeistSoundtrackPersistentObject_C|GetPDAHeist (Variables|Default|GetAs%20Heist%20Soundtrack%20Persistent%20Object)))
                                (goto _label_5)
                                (else
                                  _)))
                            (Class|SBZMusicManager|StopMusic _returnvalue_6)
                            (Class|SBZMusicManager|PlayMusic _returnvalue_6 (Variables|/Game/Mods/HeistJukebox/PDA_HeistSoundtrack.PDA_HeistSoundtrack_C|GetAudio%20Event (Variables|/Game/Mods/braidy08mods/HeistJukeboxRecode/HeistSoundtrackPersistentObject.HeistSoundtrackPersistentObject_C|GetPDAHeist (Variables|Default|GetAs%20Heist%20Soundtrack%20Persistent%20Object))) false)
                            (Variables|/Game/Mods/braidy08mods/HeistJukeboxRecode/HeistSoundtrackPersistentObject.HeistSoundtrackPersistentObject_C|SetHeistIsRTC (Variables|Default|GetAs%20Heist%20Soundtrack%20Persistent%20Object) false))
                          (:then_1
                            (goto _label_2))))
                      (else
                        (Utilities|FlowControl|Sequence
                          (:then_0
                            (goto _label_2))
                          (:then_1
                            (bind _returnvalue_9 (Actor|GetActorOfClass "/Script/Starbreeze.PD3HeistGameState"))
                            (Utilities|FlowControl|Delay 2.0)
                            (bind _outputpins (Class|PD3HeistGameState|StealthBranch _returnvalue_9))
                            (switch Utilities|FlowControl|Switch|SwitchonESBZStealthBranch _outputpins
                              (:Loud
                                (Utilities|FlowControl|Delay 0.2)
                                (goto _label_4)))))))
                    (elif (Variables|/Game/Mods/HeistJukebox/PDA_HeistSoundtrack.PDA_HeistSoundtrack_C|GetHeist%20Only (Variables|/Game/Mods/braidy08mods/HeistJukeboxRecode/HeistSoundtrackPersistentObject.HeistSoundtrackPersistentObject_C|GetPDAHeist (Variables|Default|GetAs%20Heist%20Soundtrack%20Persistent%20Object)))
                      (if (Class|SBZOnlineFunctionLibrary|IsSoloGame)
                        (if (Utilities|Enum|Equal(Enum) (Class|SBZGameStateMachineFunctionLibrary|GetGameStateMachineState) "SM_ActionPhase") :!label _label_6
                          _
                          (else
                            (Utilities|FlowControl|Delay 0.2)
                            (goto _label_6))))
                      (bind _returnvalue_10 (Class|SBZEventLibrary|GetGameEventBroker))
                      (EventDispatchers|BindEventtoOnHeistGoneLoud _returnvalue_10 (EventDispatchers|CreateEvent :!event Custom|EventOnHeistGoneLoud_0))
                      (else
                        ;[1 1 1] playsongshit
                        (if (Class|SBZOnlineFunctionLibrary|IsSoloGame)
                          (if (Utilities|Enum|Equal(Enum) (Class|SBZGameStateMachineFunctionLibrary|GetGameStateMachineState) "SM_ActionPhase") :!label _label_7
                            _
                            (else
                              (Utilities|FlowControl|Delay 0.2)
                              (goto _label_7))))
                        (Class|SBZMusicManager|StopMusic _returnvalue_4)
                        (Class|SBZMusicManager|PlayMusic _returnvalue_4 (Variables|/Game/Mods/HeistJukebox/PDA_HeistSoundtrack.PDA_HeistSoundtrack_C|GetAudio%20Event (Variables|/Game/Mods/braidy08mods/HeistJukeboxRecode/HeistSoundtrackPersistentObject.HeistSoundtrackPersistentObject_C|GetPDAHeist (Variables|Default|GetAs%20Heist%20Soundtrack%20Persistent%20Object))) false)
                        (if (Variables|/Game/Mods/HeistJukebox/PDA_HeistSoundtrack.PDA_HeistSoundtrack_C|GetStealth%20Only (Variables|/Game/Mods/braidy08mods/HeistJukeboxRecode/HeistSoundtrackPersistentObject.HeistSoundtrackPersistentObject_C|GetPDAHeist (Variables|Default|GetAs%20Heist%20Soundtrack%20Persistent%20Object)))
                          (bind _returnvalue_11 (Actor|GetActorOfClass "/Script/Starbreeze.PD3HeistGameState"))
                          (if (Utilities|Enum|Equal(Enum) (Class|PD3HeistGameState|GetCurrentHeistState _returnvalue_11) "Stealth")
                            (goto _label_2)
                            (elif (Utilities|Enum|Equal(Enum) (Class|PD3HeistGameState|GetCurrentHeistState _returnvalue_11) "Search")
                              (goto _label_2)
                              (elif (not (Variables|/Game/Mods/braidy08mods/HeistJukeboxRecode/HeistSoundtrackPersistentObject.HeistSoundtrackPersistentObject_C|GetplaylistEnabled (Variables|Default|GetAs%20Heist%20Soundtrack%20Persistent%20Object)))
                                ;[1 1 1] random assault shit
                                (Variables|/Game/Mods/braidy08mods/HeistJukeboxRecode/HeistSoundtrackPersistentObject.HeistSoundtrackPersistentObject_C|SetPDAHeist (Variables|Default|GetAs%20Heist%20Soundtrack%20Persistent%20Object) (.OutItem (Utilities|Array|Random (Variables|Default|GetPDAHeistSoundtrackarray))) :!label _label_8)
                                (if (Variables|/Game/Mods/HeistJukebox/PDA_HeistSoundtrack.PDA_HeistSoundtrack_C|GetStealth%20Only (Variables|/Game/Mods/braidy08mods/HeistJukeboxRecode/HeistSoundtrackPersistentObject.HeistSoundtrackPersistentObject_C|GetPDAHeist (Variables|Default|GetAs%20Heist%20Soundtrack%20Persistent%20Object)))
                                  (goto _label_8)
                                  (else
                                    (Class|SBZMusicManager|StopMusic _returnvalue_2)
                                    (Class|SBZMusicManager|PlayMusic _returnvalue_2 (Variables|/Game/Mods/HeistJukebox/PDA_HeistSoundtrack.PDA_HeistSoundtrack_C|GetAudio%20Event (Variables|/Game/Mods/braidy08mods/HeistJukeboxRecode/HeistSoundtrackPersistentObject.HeistSoundtrackPersistentObject_C|GetPDAHeist (Variables|Default|GetAs%20Heist%20Soundtrack%20Persistent%20Object))) false))))))
                          (elif (Variables|/Game/Mods/braidy08mods/HeistJukeboxRecode/HeistSoundtrackPersistentObject.HeistSoundtrackPersistentObject_C|GetassaultRandomSong (Variables|Default|GetAs%20Heist%20Soundtrack%20Persistent%20Object))
                            (goto _label_2)))))))))
            (:then_1
              (bind _returnvalue_12 (UserInterface|CreateWidget "/Game/Mods/LegacyHeistJukebox/WBP_CurrentSong.WBP_CurrentSong_C"))
              (bind _output_get_2 (Variables|Default|SetWBP_CurrentSong _returnvalue_12))
              (UserInterface|Viewport|AddtoViewport _returnvalue_12 9999)
              (goto _label_3))))))
    (:CastFailed
      (CallFunction|PrinttoModLoader "FAILED TO FIND PERSISTENT MOD OBJECT ON HEIST"))))

(event Input|ActionEvents|InputActionInGameMenu
  (params (Key :type Key%20Structure :default "None"))
  ;[1 1 1] need to make this work but too lazy
)

(fn ConstructionScript
  (|CallParentFunction))

(fn LoadSongs
  (bind _pdaheistsoundtrackarray (Variables|Default|GetPDAHeistSoundtrackarray))
  (Utilities|Array|Clear _pdaheistsoundtrackarray)
  (Utilities|Array|AppendArray _pdaheistsoundtrackarray (Variables|/Game/Mods/braidy08mods/HeistJukeboxRecode/HeistSoundtrackPersistentObject.HeistSoundtrackPersistentObject_C|GetPDAHeistSoundtrackarray (Variables|Default|GetAs%20Heist%20Soundtrack%20Persistent%20Object))))

(fn GetSongatIndex
  (params (Index :type Integer))
  (return (Utilities|Array|Get(acopy) (Variables|Default|GetPDAHeistSoundtrackarray) Index)))